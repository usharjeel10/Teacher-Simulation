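; Touch-controlled camera for a cheating-catching level, where the player holds on the cheating student to catch them.
; Drag input rotates the clamped view, with input disabled until SetEnableInputs is called.
; When Interact starts, a touch trace matching CheatingStd triggers a timeline FOV zoom.
; Holding fills the crosshair's radial slider over two seconds, then calls StudentCaught and resets FOV; canceling resets progress and zoom.
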(event Custom|SetCheatingStd
  (params (NewParam :type Pawn%20Object%20Reference))
  (Variables|Default|SetCheating%20Std NewParam))

(event Custom|SetEnableInputs
  (Input|EnableInput (Game|GetPlayerController 0)))

(event Input|EnhancedActionEvents|EnhancedInputActionIA_Interact
  (params (ActionValue :type Boolean) (ElapsedSeconds :type Float%20%28double-precision%29) (TriggeredSeconds :type Float%20%28double-precision%29) (InputAction :type Input%20Action%20Object%20Reference :default "/Game/inputs/IA_Interact.IA_Interact"))
  (:Started
    (if (and (Variables|Default|GetNewVar) (== (.HitActor (Collision|BreakHitResult (.HitResult (Class|PlayerController|GetHitResultUnderFingerbyChannel (Game|GetPlayerController 0) "Touch1" "TraceTypeQuery2" true)))) (Variables|Default|GetCheating%20Std)))
      (Variables|Default|SetcanZoom true)
      (bind _newtrack_0 (Timeline|Timeline PlayFromStart)
        (:Update
          (Camera|SetFieldOfView (Variables|Default|GetCamera) _newtrack_0)))))
  (:Ongoing
    (if (and (Variables|Default|GetcanZoom) (Variables|Default|GetNewVar))
      (bind _output_get (Variables|Default|SetCheatingDuration (+ (Utilities|Time|GetWorldDeltaSeconds) (Variables|Default|GetCheatingDuration))))
      (Variables|/Script/AdvancedWidgets.RadialSlider|SetValue (Variables|/Game/Test/CaughtCheating/BP/WBP/WBP_CrossHair.WBP_CrossHair_C|GetRadialSlider_64 (Variables|Default|GetWBP_CrossHair_ref)) (/ _output_get 2.0))
      (if (>= (Variables|Default|GetCheatingDuration) 2.0)
        (Variables|Default|SetCheatingDuration 0.0)
        (Default|CallStudentCaught)
        (Variables|Default|SetcanZoom false)
        (Variables|Default|SetNewVar false)
        (Camera|SetFieldOfView (Variables|Default|GetCamera) 9e+01))
      (else
        (Camera|SetFieldOfView (Variables|Default|GetCamera) 9e+01)
        (bind _output_get_2 (Variables|Default|SetCheatingDuration 0.0))
        (Variables|/Script/AdvancedWidgets.RadialSlider|SetValue (Variables|/Game/Test/CaughtCheating/BP/WBP/WBP_CrossHair.WBP_CrossHair_C|GetRadialSlider_64 (Variables|Default|GetWBP_CrossHair_ref)) _output_get_2))))
  (:Canceled
    (Variables|Default|SetCheatingDuration 0.0)
    (Variables|Default|SetcanZoom false)
    (Utilities|FlowControl|Sequence
      (:then_0
        (Timeline|Timeline Stop))
      (:then_1
        (Camera|SetFieldOfView (Variables|Default|GetCamera) 9e+01)
        (Variables|/Script/AdvancedWidgets.RadialSlider|SetValue (Variables|/Game/Test/CaughtCheating/BP/WBP/WBP_CrossHair.WBP_CrossHair_C|GetRadialSlider_64 (Variables|Default|GetWBP_CrossHair_ref)) 0.0)))))

(event EventBeginPlay
  (bind _returnvalue (Game|GetPlayerCameraManager 0))
  (bind _returnvalue_2 (UserInterface|CreateWidget "/Game/Test/CaughtCheating/BP/WBP/WBP_CrossHair.WBP_CrossHair_C"))
  (bind _output_get (Variables|Default|SetWBP_CrossHair_ref _returnvalue_2))
  (UserInterface|Viewport|AddtoViewport _output_get 0)
  (Input|DisableInput (Game|GetPlayerController 0))
  (Variables|/Script/Engine.PlayerCameraManager|SetViewYawMax _returnvalue -1.4e+02)
  (Variables|/Script/Engine.PlayerCameraManager|SetViewYawMin _returnvalue -2.2e+02)
  (Variables|/Script/Engine.PlayerCameraManager|SetViewPitchMax _returnvalue 25.0)
  (Variables|/Script/Engine.PlayerCameraManager|SetViewPitchMin _returnvalue -25.0))

(event Input|TouchEvents|InputTouch
  (params (Location :type Vector) (FingerIndex :type ETouchIndex%20Enum))
  (bind _returnvalue (Math|Vector2D|MakeVector2D (.x Location) (.y Location)))
  (bind _looksensitivity (Variables|Default|GetLookSensitivity))
  (:Pressed
    (Variables|Default|SetTouchStartPos _returnvalue))
  (:Moved
    (bind _output_get (Variables|Default|SetTouchEndPos _returnvalue))
    (Pawn|Input|AddControllerYawInput (* (.x (- _output_get (Variables|Default|GetTouchStartPos))) _looksensitivity))
    (Pawn|Input|AddControllerPitchInput (* (.y (- _output_get (Variables|Default|GetTouchStartPos))) _looksensitivity))
    (Variables|Default|SetTouchStartPos (Variables|Default|GetTouchEndPos))))

(fn ConstructionScript)