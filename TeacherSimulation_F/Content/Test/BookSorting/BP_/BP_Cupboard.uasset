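; Cupboard actor for a book-sorting puzzle that holds a stack of up to six books at preset slot positions.
; Added books snap into the next slot; a check pass drops books whose state has changed and flags only the last one as OnTop.
; A fullness check counts consecutive same-color books and, at six, locks the cupboard and calls the GMIP game instance to load a level.
; Construction hides or removes an optional hand-arrow component.
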(event Custom|AddBookToCupboard
  (params (Book :type BP%20Book%20Object%20Reference))
  (if (not (>= (Utilities|Array|Length (Variables|Default|GetBookSlot)) 6))
    (bind _returnvalue (Utilities|Array|AddUnique (Variables|Default|GetBookSlot) Book))
    (if (== _returnvalue (Variables|Default|GetCupboardIndex))
      (Transformation|SetActorLocation Book (Utilities|Array|Get(acopy) (Variables|Default|GetBookSlotPos) (Variables|Default|GetCupboardIndex)) false false)
      (bind _result (Math|Integer|IncrementInt (Variables|Default|GetCupboardIndex))
        (:%20%20
          (Variables|Default|SetCupboardIndex _result)
          (Default|SetState Book (Variables|Default|GetNewVar)))))))

(event Custom|CheckCupboard
  (bind _bookslot (Variables|Default|GetBookSlot))
  (if (> (Utilities|Array|Length _bookslot) 0)
    (for (_array_element _array_index) _bookslot
      (bind _asbp_book (Utilities|Casting|CastToBP_Book _array_element))
      (if (not (Utilities|Enum|Equal(Enum) (Variables|/Game/Test/BookSorting/BP_/BP_Book.BP_Book_C|GetE_BS _asbp_book) (Variables|Default|GetNewVar)))
        (Utilities|Array|RemoveItem (Variables|Default|GetBookSlot) (Utilities|Array|Get(acopy) (Variables|Default|GetBookSlot) _array_index))
        (bind _result (Math|Integer|DecrementInt (Variables|Default|GetCupboardIndex))
          (:%20%20
            (Variables|Default|SetCupboardIndex _result)))))
    (if (> (- (Variables|Default|GetCupboardIndex) 1) -1)
      (for _array_element_2 (Variables|Default|GetBookSlot)
        (Variables|/Game/Test/BookSorting/BP_/BP_Book.BP_Book_C|Set?OnTop _array_element_2 false))
      (if (Variables|Default|GetCaChechBooks)
        (Variables|/Game/Test/BookSorting/BP_/BP_Book.BP_Book_C|Set?OnTop (Utilities|Array|Get(acopy) (Variables|Default|GetBookSlot) (- (Variables|Default|GetCupboardIndex) 1)) true)))))

(event Custom|checkCupboardIsFull?
  (for _array_element (Variables|Default|GetBookSlot)
    (switch Utilities|FlowControl|Switch|SwitchonBookCategory (Variables|/Game/Test/BookSorting/BP_/BP_Book.BP_Book_C|GetbookCatagory _array_element)
      (:NewEnumerator0
        (Variables|Default|SetRedcounter (+ (Variables|Default|GetRedcounter) 1))
        (Variables|Default|SetGreenCounter 0)
        (Variables|Default|SetBlueCounter 0))
      (:NewEnumerator1
        (Variables|Default|SetGreenCounter (+ (Variables|Default|GetGreenCounter) 1))
        (Variables|Default|SetRedcounter 0)
        (Variables|Default|SetBlueCounter 0))
      (:NewEnumerator2
        (Variables|Default|SetBlueCounter (+ (Variables|Default|GetBlueCounter) 1))
        (Variables|Default|SetGreenCounter 0)
        (Variables|Default|SetRedcounter 0))))
  (if (Math|Boolean|ORBoolean (== (Variables|Default|GetRedcounter) 6) (== (Variables|Default|GetGreenCounter) 6) (== (Variables|Default|GetBlueCounter) 6))
    (if (== (Variables|Default|GetRedcounter) 6)
      (Development|PrintString "CupBoard Is Full With Specific Book Type Red")
      (Variables|Default|SetCaChechBooks false)
      (Variables|Default|SetGreenCounter 0)
      (Variables|Default|SetBlueCounter 0)
      (Variables|Default|SetRedcounter 0)
      (Variables|/Game/Test/BookSorting/BP_/BP_Book.BP_Book_C|Set?OnTop (Utilities|Array|Get(acopy) (Variables|Default|GetBookSlot) (- (Variables|Default|GetCupboardIndex) 1)) false)
      (bind _asgmip (Utilities|Casting|CastToGMIP (Game|GetGameInstance)))
      (Default|LoadLevelforBookSorting _asgmip)
      (elif (== (Variables|Default|GetGreenCounter) 6)
        (Development|PrintString "CupBoard Is Full With Specific Book Type Green")
        (Variables|Default|SetCaChechBooks false)
        (Variables|Default|SetGreenCounter 0)
        (Variables|Default|SetBlueCounter 0)
        (Variables|Default|SetRedcounter 0)
        (Variables|/Game/Test/BookSorting/BP_/BP_Book.BP_Book_C|Set?OnTop (Utilities|Array|Get(acopy) (Variables|Default|GetBookSlot) (- (Variables|Default|GetCupboardIndex) 1)) false)
        (bind _asgmip_2 (Utilities|Casting|CastToGMIP (Game|GetGameInstance)))
        (Default|LoadLevelforBookSorting _asgmip_2)
        (elif (== (Variables|Default|GetBlueCounter) 6)
          (Development|PrintString "CupBoard Is Full With Specific Book Type Blue")
          (Variables|Default|SetCaChechBooks false)
          (Variables|Default|SetGreenCounter 0)
          (Variables|Default|SetBlueCounter 0)
          (Variables|Default|SetRedcounter 0)
          (Variables|/Game/Test/BookSorting/BP_/BP_Book.BP_Book_C|Set?OnTop (Utilities|Array|Get(acopy) (Variables|Default|GetBookSlot) (- (Variables|Default|GetCupboardIndex) 1)) false)
          (bind _asgmip_3 (Utilities|Casting|CastToGMIP (Game|GetGameInstance)))
          (Default|LoadLevelforBookSorting _asgmip_3))))
    (else
      (Variables|Default|SetGreenCounter 0)
      (Variables|Default|SetBlueCounter 0)
      (Variables|Default|SetRedcounter 0))))

(fn ConstructionScript
  (if (Variables|Default|Get?containHandArrow)
    (if (Variables|Default|GethideHand)
      (Rendering|SetVisibility (Variables|Default|Gethand) false false))
    (else
      (Components|DestroyComponent (Variables|Default|Gethand)))))