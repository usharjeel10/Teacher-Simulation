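; Antonio, a KEKOS student character in a classroom quiz who can sit, stand, cheat, offer an answer and be caught.
; Events play head-mesh animations and toggle the arrow and answer-box widgets.
; On BeginPlay it caches row q1 of DT_QuestionAnswers; when selected, it writes the indexed answer once and updates true/false answer flags.
; When caught, it slides away with a rotation after a delay, then destroys itself.
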(event Custom|studentStateInClassroom
  (params (selectState :type E_Std_Anim_State%20Enum :default "NewEnumerator0"))
  ;[0 0 0 0.5] SetStudentAnimation
  (switch Utilities|FlowControl|Switch|SwitchonE_Std_Anim_State selectState
    (:NewEnumerator0
      (Variables|Default|SetAnimOnBeginPlay "/Game/Mixamo/Animation/F_Sitting_Idle.F_Sitting_Idle"))
    (:NewEnumerator1
      (Variables|Default|SetAnimOnBeginPlay "/Game/Mixamo/Animation/F_Sit_To_Stand.F_Sit_To_Stand"))
    (:NewEnumerator2
      (Variables|Default|SetAnimOnBeginPlay "/Game/Mixamo/Animation/F_Stand_To_Sit.F_Stand_To_Sit")))
  (Components|Animation|PlayAnimation (Variables|Default|GetHEAD) (Variables|Default|GetAnimOnBeginPlay) false))

(event Custom|findStudentAndDisplayArrow
  (params (NewParam :type Byte) (Tries :type Integer))
  ;[0 0 0 0.5] EnableAnswersBoxONStudents
  (Variables|Default|SetTries Tries)
  (Variables|Default|SetCan%20Stand true)
  (Development|SetHiddeninGame (Variables|Default|GetWidget) false false)
  (Variables|Default|SetE_AnswerIndex (Utilities|Enum|ByteToEnumStudentAnswerIndex NewParam))
  (Utilities|FlowControl|DoOnce false
    (:Completed
      ;[0 0 0 0.5] AddAnswersToStudents
      (Rendering|Components|TextRender|SetText (Variables|/Game/UserWidget/WBP_AnswerBox.WBP_AnswerBox_C|GetTextBlock_250 (stale EventBeginPlay _aswbp_answer_box)) (Utilities|Select :Index (Variables|Default|GetE_AnswerIndex) :NewEnumerator0 (.answer1 (.ans (stale EventBeginPlay _returnvalue))) :NewEnumerator1 (.answer2 (.ans (stale EventBeginPlay _returnvalue))) :NewEnumerator2 (.answer3 (.ans (stale EventBeginPlay _returnvalue))) :NewEnumerator3 (.answer4 (.ans (stale EventBeginPlay _returnvalue)))))
      ;[0 0 0 0.5] GetStudentWrongAndTrueAnswer
      (switch Utilities|FlowControl|Switch|SwitchonStudentAnswerIndex (Variables|Default|GetE_AnswerIndex)
        (:NewEnumerator0
          (Variables|Default|SetFalse%20Answer false :!label _label))
        (:NewEnumerator1
          (Variables|Default|SetTrue%20Answer false))
        (:NewEnumerator2
          (goto _label))
        (:NewEnumerator3
          (goto _label))))))

(event Custom|disable%20Arrow
  ;[0 0 0 0.5] Disable Arrow When Student Stand
  (Development|SetHiddeninGame (Variables|Default|GetWidget) true false))

(event Custom|ShowAnswerBox
  ;[0 0 0 0.5] Show Answers Box
  (Variables|Default|SetCan%20Stand false)
  (Utilities|FlowControl|Delay 2.0)
  (Development|SetHiddeninGame (Variables|Default|GetW_answerBox) false false))

(event Custom|SetStudentCheatingAnim
  (Components|Animation|PlayAnimation (Variables|Default|GetHEAD) "/Game/Mixamo/Animation/F_Cheating.F_Cheating" false))

(event Custom|CaughtStudent
  (Utilities|FlowControl|Delay 1.0)
  (Components|MoveComponentTo (Variables|Default|GetCapsule) (+ (Transformation|GetActorLocation) "0.000000,-500.000000,0.000000") "0.000000,-90.000000,0.000000" false false 0.7 false)
  (Actor|DestroyActor))

(event EventBeginPlay
  ;[0 0 0 0.5] Animation&AnswersRef(DataTable)
  (Components|Animation|PlayAnimation (Variables|Default|GetHEAD) "/Game/Mixamo/Animation/F_Sitting_Idle.F_Sitting_Idle" true)
  (bind _aswbp_answer_box (Utilities|Casting|CastToWBP_AnswerBox (UserInterface|GetUserWidgetObject (Variables|Default|GetW_answerBox))))
  (bind _aspc_level_1 (Utilities|Casting|CastToPC_Level1 (Game|GetPlayerController 0)))
  (Variables|Default|SetPC%20Level%201 _aspc_level_1)
  ;[0 0 0 0.5] AddAnswersToStudents
  (bind _returnvalue (Utilities|GetDataTableRow "/Game/Blueprints/dataTables/DT_QuestionAnswers.DT_QuestionAnswers" "q1")))

(fn ConstructionScript
  (|CallParentFunction)
  (Development|SetHiddeninGame (Variables|Default|GetWidget) true false)
  (Development|SetHiddeninGame (Variables|Default|GetW_answerBox) true false))