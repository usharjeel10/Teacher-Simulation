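; Classroom student for the Level 1 quiz, showing an answer that the player judges right or wrong.
; Construction assembles its look from a student data table; BeginPlay uses the level1 save to choose the tutorial or question number.
; Selection shows an arrow and fills the answer widget from a question table, with answer 2 always correct.
; checkAnswer compares the verdict, plays reactions and reports good or bad choices with progress.
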(event Custom|studentStateInClassroom
  (params (selectState :type E_Std_Anim_State%20Enum :default "NewEnumerator0"))
  ;[0 0 0 0.5] SetStudentAnimation
  (bind _f_student_animation (Variables|Default|GetF_Student%20Animation)
    (:then
      (Default|PlayState _f_student_animation selectState))
    (:else)))

(event Custom|findStudentAndDisplayArrow
  (params (NewParam :type Byte) (Tries :type Integer))
  (bind _pc_level_1 (Variables|Default|GetPC%20Level%201))
  (bind _pc_level_1_2 (Variables|Default|GetPC%20Level%201))
  (bind _gameplaywbp_ref (Variables|/Game/CoreComponents/GameplayGameMode/PC_Level1.PC_Level1_C|GetGamePlayWBP_ref _pc_level_1))
  (bind _gameplaywbp_ref_2 (Variables|/Game/CoreComponents/GameplayGameMode/PC_Level1.PC_Level1_C|GetGamePlayWBP_ref _pc_level_1_2))
  ;[0 0 0 0.5] EnableAnswersBoxONStudents
  (Default|PlayState (Variables|Default|GetF_Student%20Animation) "NewEnumerator15")
  (Variables|Default|SetTries Tries)
  (Variables|Default|SetcanStand true)
  (Rendering|SetVisibility (Variables|Default|GetArrow_Widget) true false)
  (Variables|Default|SetE_AnswerIndex (Utilities|Enum|ByteToEnumStudentAnswerIndex NewParam))
  (Utilities|FlowControl|DoOnce false :!label _label
    (:Completed
      (if (== (Variables|Default|Get?IsTutorialLevel) 0)
        (Utilities|FlowControl|FlipFlop
          (:A
            (Variables|/Script/UMG.Widget|SetVisibility (Variables|/Game/UserWidget/gamePlayerWBPlevel01.gamePlayerWBPlevel01_C|GetHand1 _gameplaywbp_ref) "Visible")
            (Widget|SetIsEnabled (Variables|/Game/UserWidget/gamePlayerWBPlevel01.gamePlayerWBPlevel01_C|GetTickBtn _gameplaywbp_ref) false)
            (UserInterface|Animation|PlayAnimation _gameplaywbp_ref (Variables|/Game/UserWidget/gamePlayerWBPlevel01.gamePlayerWBPlevel01_C|GetRightHandAnim _gameplaywbp_ref) 0.0 0 "Forward" 1.0 false)
            (Widget|SetIsEnabled (Variables|/Game/UserWidget/gamePlayerWBPlevel01.gamePlayerWBPlevel01_C|GetCrossBtn _gameplaywbp_ref) true)
            (Rendering|Components|TextRender|SetText (Variables|/Game/UserWidget/WBP_AnswerBox.WBP_AnswerBox_C|GetTextBlock_250 (stale EventBeginPlay _aswbp_answer_box)) "Cow")
            (goto _label Reset))
          (:B
            (Variables|/Script/UMG.Widget|SetVisibility (Variables|/Game/UserWidget/gamePlayerWBPlevel01.gamePlayerWBPlevel01_C|GetHand2 _gameplaywbp_ref_2) "Visible")
            (Widget|SetIsEnabled (Variables|/Game/UserWidget/gamePlayerWBPlevel01.gamePlayerWBPlevel01_C|GetCrossBtn _gameplaywbp_ref_2) false)
            (Widget|SetIsEnabled (Variables|/Game/UserWidget/gamePlayerWBPlevel01.gamePlayerWBPlevel01_C|GetTickBtn _gameplaywbp_ref_2) true)
            (UserInterface|Animation|PlayAnimation _gameplaywbp_ref_2 (Variables|/Game/UserWidget/gamePlayerWBPlevel01.gamePlayerWBPlevel01_C|GetLeftHandAnim _gameplaywbp_ref_2) 0.0 0 "Forward" 1.0 false)
            (Variables|/Script/UMG.Widget|SetVisibility (Variables|/Game/UserWidget/gamePlayerWBPlevel01.gamePlayerWBPlevel01_C|GetHand1 _gameplaywbp_ref_2) "Hidden")
            (Rendering|Components|TextRender|SetText (Variables|/Game/UserWidget/WBP_AnswerBox.WBP_AnswerBox_C|GetTextBlock_250 (stale EventBeginPlay _aswbp_answer_box)) "Fragmile")
            (goto _label Reset)))
        (else
          ;[0 0 0 0.5] AddAnswersToStudents
          (bind _returnvalue (Utilities|GetDataTableRow "/Game/Blueprints/dataTables/DT_QuestionAnswers.DT_QuestionAnswers" (Utilities|String|StringToName (Utilities|String|ToString(Integer) (Variables|Default|Get?IsTutorialLevel))))
            (:then
              (Rendering|Components|TextRender|SetText (Variables|/Game/UserWidget/WBP_AnswerBox.WBP_AnswerBox_C|GetTextBlock_250 (stale EventBeginPlay _aswbp_answer_box)) (Utilities|Select :Index (Variables|Default|GetE_AnswerIndex) :NewEnumerator0 (.answer1 (.ans _returnvalue)) :NewEnumerator1 (.answer2 (.ans _returnvalue)) :NewEnumerator2 (.answer3 (.ans _returnvalue)) :NewEnumerator3 (.answer4 (.ans _returnvalue))))
              ;[0 0 0 0.5] GetStudentWrongAndTrueAnswer
              (switch Utilities|FlowControl|Switch|SwitchonStudentAnswerIndex (Variables|Default|GetE_AnswerIndex)
                (:NewEnumerator0
                  (Variables|Default|SetFalseAnswer true :!label _label_2))
                (:NewEnumerator1
                  (Variables|Default|SetTrueAnswer true))
                (:NewEnumerator2
                  (goto _label_2))
                (:NewEnumerator3
                  (goto _label_2)))
              (Rendering|SetVisibility (Variables|Default|GetArrow_Widget) true false))))))))

(event Custom|disable%20Arrow
  ;[0 0 0 0.5] Disable Arrow When Student Stand
  (Rendering|SetVisibility (Variables|Default|GetArrow_Widget) false false)
  (Default|PlayState (Variables|Default|GetF_Student%20Animation) "NewEnumerator0"))

(event Custom|AddProgressBarLength
  (params (PogressBar :type Float%20%28double-precision%29) (student%20AnswerWrong :type Boolean))
  ;[0 0 0 0.5] Check Answer (if true then complete gama. base on the answers play animations and stop the game)............... For Level  01
)

(event Custom|checkAnswer
  (params (True :type Boolean))
  (bind _progressbarlength (Variables|Default|GetProgressBarLength))
  (bind _pc_level_1 (Variables|Default|GetPC%20Level%201))
  (bind _gameplaywbp_ref (Variables|/Game/CoreComponents/GameplayGameMode/PC_Level1.PC_Level1_C|GetGamePlayWBP_ref _pc_level_1))
  ;[0 0 0 0.5] Check Answer (if true then complete gama. base on the answers play animations and stop the game)............... For Level  01
  (if True
    (if (Variables|Default|GetTrueAnswer)
      (Variables|/Game/CoreComponents/GameplayGameMode/PC_Level1.PC_Level1_C|SetCanUnfocusOnStudent (Variables|Default|GetPC%20Level%201) false)
      (Default|PlayState (Variables|Default|GetF_Student%20Animation) "NewEnumerator9")
      (Default|CallOnChoice _progressbarlength false)
      (Development|PrintString "complete Level/HappyAnimation" true true "(R=0.000000,G=1.000000,B=0.141202,A=1.000000)" 14.0 :!label _label)
      (Utilities|FlowControl|Delay 2.0)
      (Rendering|SetVisibility (Variables|Default|GetW_answerBox) false false)
      (else
        (if (Variables|Default|GetFalseAnswer)
          (Default|PlayState (Variables|Default|GetF_Student%20Animation) "NewEnumerator9")
          (Default|CallOnBadChoice _progressbarlength)
          (else
            (Default|PlayState (Variables|Default|GetF_Student%20Animation) "NewEnumerator9")
            (Default|CompleteTutorialQuestions (Variables|/Game/CoreComponents/GameplayGameMode/PC_Level1.PC_Level1_C|GetST_ActorRef (Variables|Default|GetPC%20Level%201)))
            (Variables|/Script/UMG.Widget|SetVisibility (Variables|/Game/UserWidget/gamePlayerWBPlevel01.gamePlayerWBPlevel01_C|GetHand1 _gameplaywbp_ref) "Hidden")
            (Variables|/Script/UMG.Widget|SetVisibility (Variables|/Game/UserWidget/gamePlayerWBPlevel01.gamePlayerWBPlevel01_C|GetHand2 _gameplaywbp_ref) "Hidden")
            (Default|CallOnChoice _progressbarlength false :!label _label_2)))
        (Rendering|SetVisibility (Variables|Default|GetW_answerBox) false false :!label _label_3)))
    (elif (Variables|Default|GetTrueAnswer)
      (Variables|/Game/CoreComponents/GameplayGameMode/PC_Level1.PC_Level1_C|SetCanUnfocusOnStudent (Variables|Default|GetPC%20Level%201) false)
      (Default|PlayState (Variables|Default|GetF_Student%20Animation) "NewEnumerator10")
      (Default|CallOnBadChoice _progressbarlength)
      (goto _label)
      (elif (Variables|Default|GetFalseAnswer)
        (Default|PlayState (Variables|Default|GetF_Student%20Animation) "NewEnumerator10")
        (Default|CallOnChoice _progressbarlength true)
        (goto _label_3)
        (else
          (Default|PlayState (Variables|Default|GetF_Student%20Animation) "NewEnumerator10")
          (goto _label_2))))))

(event Custom|handsDownAnimation
  (Default|PlayState (Variables|Default|GetF_Student%20Animation) "NewEnumerator0"))

(event Custom|ShowAnswerBox
  ;[0 0 0 0.5] Show Answers Box
  (Utilities|FlowControl|Sequence
    (:then_0
      (Utilities|FlowControl|DoOnce false
        (:Completed
          (Default|DisableInstructionUI (Variables|/Game/CoreComponents/GameplayGameMode/PC_Level1.PC_Level1_C|GetGamePlayWBP_ref (Variables|Default|GetPC%20Level%201))))))
    (:then_1
      (Variables|Default|SetcanStand false)
      (Utilities|FlowControl|Delay 2.0)
      (Rendering|SetVisibility (Variables|Default|GetW_answerBox) true false))))

(event Custom|CaughtStudent
  (Utilities|FlowControl|Delay 1.0)
  (Components|MoveComponentTo (Variables|Default|GetCapsule) (+ (Transformation|GetActorLocation) "0.000000,-500.000000,0.000000") "0.000000,-90.000000,0.000000" false false 0.7 false)
  (Actor|DestroyActor))

(event EventBeginPlay
  ;[0 0 0 0.5] Animation&AnswersRef(DataTable)
  (bind _aspc_level_1 (Utilities|Casting|CastToPC_Level1 (Game|GetPlayerController 0))
    (:then
      (Variables|Default|SetPC%20Level%201 _aspc_level_1)
      (Utilities|FlowControl|Sequence
        (:then_0
          (bind _returnvalue (SaveGame|DoesSaveGameExist "level1"))
          (if _returnvalue
            (bind _returnvalue_2 (SaveGame|LoadGamefromSlot "level1"))
            (bind _asbp_save (Utilities|Casting|CastToBP_Save _returnvalue_2))
            (bind _output_get (Variables|Default|SetAs%20BP%20Save _asbp_save))
            (SaveGame|SaveGametoSlot _output_get "level1")
            (bind _as_bp_save (Variables|Default|GetAs%20BP%20Save)
              (:then
                (if (> (Variables|/Game/Blueprints/SaveGame/BP_Save.BP_Save_C|GetCurrentQuestion _as_bp_save) 0)
                  (if (>= (Variables|/Game/Blueprints/SaveGame/BP_Save.BP_Save_C|GetCurrentQuestion _as_bp_save) (Variables|Default|GetTotalQuestions))
                    (Utilities|FlowControl|Delay 0.2)
                    (Variables|Default|Set?IsTutorialLevel (Variables|/Game/CoreComponents/GameplayGameMode/PC_Level1.PC_Level1_C|GetRandomQuestionNo (Variables|Default|GetPC%20Level%201)))
                    (else
                      (Variables|Default|Set?IsTutorialLevel (+ (Variables|/Game/Blueprints/SaveGame/BP_Save.BP_Save_C|GetCurrentQuestion _as_bp_save) 1))))
                  (Variables|Default|SetProgressBarLength 0.25)
                  (else
                    (Variables|Default|Set?IsTutorialLevel 0)
                    (Variables|Default|SetProgressBarLength 0.125))))
              (:else))
            (else
              (bind _returnvalue_3 (SaveGame|CreateSaveGameObject "/Game/Blueprints/SaveGame/BP_Save.BP_Save_C"))
              (SaveGame|SaveGametoSlot _returnvalue_3 "level1"))))
        (:then_1
          (Utilities|FlowControl|Delay 0.5)
          (bind _asf_student_animation (Utilities|Casting|CastToF_StudentAnimation (Components|SkeletalMesh|GetAnimInstance (Variables|Default|GetHead))))
          (Variables|Default|SetF_Student%20Animation _asf_student_animation)
          (bind _aswbp_answer_box (Utilities|Casting|CastToWBP_AnswerBox (UserInterface|GetUserWidgetObject (Variables|Default|GetW_answerBox))))
          (Default|GetQuestionNo (Variables|Default|GetPC%20Level%201) (Variables|Default|Get?IsTutorialLevel)))))
    (:CastFailed
      (bind _asf_student_animation_2 (Utilities|Casting|CastToF_StudentAnimation (Components|SkeletalMesh|GetAnimInstance (Variables|Default|GetHead))))
      (Variables|Default|SetF_Student%20Animation _asf_student_animation_2))))

(fn ConstructionScript
  (Variables|Default|SetCurrent%20Std%20Uniform%20Index (Utilities|Array|Get(acopy) (Variables|Default|GetRandomStudentWuniform) (Variables|Default|GetCurrent%20Std%20Uniform%20Index)))
  (Rendering|SetVisibility (Variables|Default|GetArrow_Widget) false false)
  (Rendering|SetVisibility (Variables|Default|GetW_answerBox) false false)
  (|CallParentFunction)
  (bind _returnvalue (Utilities|GetDataTableRow "/Game/Blueprints/structure/STdUniform/STD_DATA_TABLE.STD_DATA_TABLE" (Utilities|String|StringToName (Utilities|String|ToString(Integer) (Variables|Default|GetCurrent%20Std%20Uniform%20Index))))
    (:then
      (Variables|Default|SetSkinMaterial (.skinColour (Utilities|Struct|BreakStd_Cloths _returnvalue)))
      (Variables|Default|SetTorsoMesh (.TorsoMesh (Utilities|Struct|BreakStd_Cloths _returnvalue)))
      (Variables|Default|SetTorsoMaterial (.TorsoMaterialArray (Utilities|Struct|BreakStd_Cloths _returnvalue)))
      (Variables|Default|SetLegsMesh (.LegMesh (Utilities|Struct|BreakStd_Cloths _returnvalue)))
      (Variables|Default|SetLegsMaterial (.LegMaterialArray (Utilities|Struct|BreakStd_Cloths _returnvalue)))
      (Variables|Default|SetHandsMesh (.HandMesh (Utilities|Struct|BreakStd_Cloths _returnvalue)))
      (Variables|Default|SetHandsMaterial (.HandMaterial (Utilities|Struct|BreakStd_Cloths _returnvalue)))
      (Variables|Default|SetFeetsMesh (.FeetMesh (Utilities|Struct|BreakStd_Cloths _returnvalue)))
      (Variables|Default|SetFeetsMaterial (.FeetMaterial (Utilities|Struct|BreakStd_Cloths _returnvalue)))
      (Variables|Default|SetFullTorsoMesh (.FullTorsoMesh (Utilities|Struct|BreakStd_Cloths _returnvalue)))
      (Variables|Default|SetFullTorsoMaterial (.FullTorsoMaterialArray (Utilities|Struct|BreakStd_Cloths _returnvalue)))
      (Variables|Default|SetTorsoPropMesh (.TorsoPropMesh (Utilities|Struct|BreakStd_Cloths _returnvalue)))
      (Variables|Default|SetTorsoPropMaterial (.TorsoPropMaterialArray (Utilities|Struct|BreakStd_Cloths _returnvalue)))
      (Variables|Default|SetCapMesh (.capMesh (Utilities|Struct|BreakStd_Cloths _returnvalue)))
      (Variables|Default|SetCapMaterial (.CapMaterial (Utilities|Struct|BreakStd_Cloths _returnvalue)))
      (Variables|Default|SetGlassesMesh (.GlassesMesh (Utilities|Struct|BreakStd_Cloths _returnvalue)))
      (Variables|Default|SetGlassesMaterial (.GlassesMaterial (Utilities|Struct|BreakStd_Cloths _returnvalue)))
      (Variables|Default|SetHairMesh (.HairMesh (Utilities|Struct|BreakStd_Cloths _returnvalue)))
      (Variables|Default|SetHairColor (.HairColor (Utilities|Struct|BreakStd_Cloths _returnvalue)))
      (Variables|Default|SetEyebrowsMesh (.EyeBrowMesh (Utilities|Struct|BreakStd_Cloths _returnvalue)))
      (Variables|Default|SetEyebrowsColor (.EyeBrowColor (Utilities|Struct|BreakStd_Cloths _returnvalue))))))