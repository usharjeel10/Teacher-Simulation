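; Pen actor for an ink pot filling interaction: one of three pencil variants moves to its idle position, uncaps and accepts input.
; Holding TestHoldBtn drives timelines that dip the pen and pull its back piece, with repeating camera shake.
; Releasing early reports fill progress and reverses the dip; completing disables input and recaps the pen.
; FlipFlops reuse timeline completions to send the pen back and call the next one.
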(event Custom|CustomEvent
  (Camera|PlayWorldCameraShake "/Game/inputs/pencil_and_PencilCameraShake.pencil_and_PencilCameraShake_C" (Transformation|GetActorLocation (Variables|Default|Getbp_cameraRef)) 0.0 5e+02))

(event Custom|PenProgress
  (params (Progress :type Float%20%28double-precision%29)))

(event Input|EnhancedActionEvents|EnhancedInputActionTestHoldBtn
  (params (ActionValue :type Boolean) (ElapsedSeconds :type Float%20%28double-precision%29) (TriggeredSeconds :type Float%20%28double-precision%29) (InputAction :type Input%20Action%20Object%20Reference :default "/Game/inputs/TestHoldBtn.TestHoldBtn"))
  (:Started
    (Variables|Default|SetReady true)
    (bind (_direction _newtrack_0 _newtrack_2) (Timeline|MovePenToInkPot Play)
      (:Update
        (Transformation|SetActorLocationAndRotation _newtrack_0 (Math|Rotator|MakeRotator (.x _newtrack_2) (.y _newtrack_2) (.z _newtrack_2))))
      (:Finished
        (if (Variables|Default|GetReady)
          (Utilities|FlowControl|Sequence
            (:then_0
              (bind _newtrack_0_2 (Timeline|PullPenBack Play)
                (:Update
                  (Transformation|SetRelativeLocation (Variables|Default|GetPenBack) (Math|Vector|MakeVector 0.0 0.0 _newtrack_0_2) false false))
                (:Finished
                  (Utilities|FlowControl|Sequence
                    (:then_0
                      (Variables|Default|SetReady false)
                      (Variables|Default|SetFillThePen true)
                      (Input|DisableInput (Game|GetPlayerController 0))
                      (Default|CallPenFillEvent 0.0)
                      (Timeline|MovePenToInkPot ReverseFromEnd))
                    (:then_1
                      (Utilities|Time|ClearandInvalidateTimerbyHandle (Variables|Default|GetTimerEvent)))))))
            (:then_1
              (Camera|PlayWorldCameraShake "/Game/inputs/pencil_and_PencilCameraShake.pencil_and_PencilCameraShake_C" (Transformation|GetActorLocation (Variables|Default|Getbp_cameraRef)) 0.0 5e+02)
              (bind _returnvalue (Utilities|Time|SetTimerbyEvent (delegate Custom|CustomEvent) 0.5 true))
              (Variables|Default|SetTimerEvent _returnvalue)))
          (elif (Variables|Default|GetFillThePen)
            (bind _newtrack_0_3 (Timeline|RemovePenCover ReverseFromEnd)
              (:Update
                (Transformation|SetRelativeLocation (Variables|Default|GetPenCover) (Math|Vector|MakeVector _newtrack_0_3 0.56 0.0) false false))
              (:Finished
                (Utilities|FlowControl|FlipFlop
                  (:A
                    (Input|EnableInput (Game|GetPlayerController 0)))
                  (:B
                    (switch Utilities|FlowControl|Switch|SwitchonE_PencilNo (stale EventMoveobjecttoIdlePos NewParam)
                      (:NewEnumerator0
                        (bind (_direction_2 _newtrack_1 _newtrack_2_2) (Timeline|MoveToIdleTimeLine ReverseFromEnd)
                          (:Update
                            (Transformation|SetActorLocationAndRotation _newtrack_1 (Math|Rotator|MakeRotator (.x _newtrack_2_2) (.y _newtrack_2_2) (.z _newtrack_2_2))))
                          (:Finished
                            (Utilities|FlowControl|FlipFlop :!label _label
                              (:A
                                (Utilities|FlowControl|Delay 0.3)
                                (Timeline|RemovePenCover PlayFromStart))
                              (:B
                                (Default|CallNextPenMovetoIdle))))))
                      (:NewEnumerator1
                        (bind (_direction_3 _newtrack_1_2 _newtrack_2_3) (Timeline|Timeline_1 ReverseFromEnd)
                          (:Update
                            (Transformation|SetActorLocationAndRotation _newtrack_1_2 (Math|Rotator|MakeRotator (.x _newtrack_2_3) (.y _newtrack_2_3) (.z _newtrack_2_3))))
                          (:Finished
                            (goto _label))))
                      (:NewEnumerator2
                        (bind (_direction_4 _newtrack_1_3 _newtrack_2_4) (Timeline|Timeline ReverseFromEnd)
                          (:Update
                            (Transformation|SetActorLocationAndRotation _newtrack_1_3 (Math|Rotator|MakeRotator (.x _newtrack_2_4) (.y _newtrack_2_4) (.z _newtrack_2_4))))
                          (:Finished
                            (goto _label))))))))))))))
  (:Canceled
    (Default|CallPenFillEvent (.z (Variables|/Script/Engine.SceneComponent|GetRelativeLocation (Variables|Default|GetPenBack))))
    (Variables|Default|SetReady false)
    (Utilities|FlowControl|Sequence
      (:then_0
        (Timeline|MovePenToInkPot Reverse))
      (:then_1
        (Utilities|Time|ClearandInvalidateTimerbyHandle (Variables|Default|GetTimerEvent))
        (Timeline|PullPenBack Stop)))))

(event EventMoveobjecttoIdlePos
  (params (NewParam :type E_PencilNo%20Enum :default "NewEnumerator0"))
  (bind _returnvalue (Actor|GetActorOfClass "/Game/Test/InkPot/BluePrint/BP_Camera_02.BP_Camera_02_C"))
  (Variables|Default|SetBP_CameraRef _returnvalue)
  (switch Utilities|FlowControl|Switch|SwitchonE_PencilNo NewParam
    (:NewEnumerator0
      (bind (_direction _newtrack_1 _newtrack_2) (Timeline|MoveToIdleTimeLine PlayFromStart)
        (:Update
          (Transformation|SetActorLocationAndRotation _newtrack_1 (Math|Rotator|MakeRotator (.x _newtrack_2) (.y _newtrack_2) (.z _newtrack_2))))
        (:Finished
          (Utilities|FlowControl|FlipFlop :!label _label
            (:A
              (Utilities|FlowControl|Delay 0.3)
              (bind _newtrack_0 (Timeline|RemovePenCover PlayFromStart)
                (:Update
                  (Transformation|SetRelativeLocation (Variables|Default|GetPenCover) (Math|Vector|MakeVector _newtrack_0 0.56 0.0) false false))
                (:Finished
                  (Utilities|FlowControl|FlipFlop
                    (:A
                      (Input|EnableInput (Game|GetPlayerController 0)))
                    (:B
                      (switch Utilities|FlowControl|Switch|SwitchonE_PencilNo NewParam
                        (:NewEnumerator0
                          (Timeline|MoveToIdleTimeLine ReverseFromEnd))
                        (:NewEnumerator1
                          (bind (_direction_2 _newtrack_1_2 _newtrack_2_2) (Timeline|Timeline_1 ReverseFromEnd)
                            (:Update
                              (Transformation|SetActorLocationAndRotation _newtrack_1_2 (Math|Rotator|MakeRotator (.x _newtrack_2_2) (.y _newtrack_2_2) (.z _newtrack_2_2))))
                            (:Finished
                              (goto _label))))
                        (:NewEnumerator2
                          (bind (_direction_3 _newtrack_1_3 _newtrack_2_3) (Timeline|Timeline ReverseFromEnd)
                            (:Update
                              (Transformation|SetActorLocationAndRotation _newtrack_1_3 (Math|Rotator|MakeRotator (.x _newtrack_2_3) (.y _newtrack_2_3) (.z _newtrack_2_3))))
                            (:Finished
                              (goto _label))))))))))
            (:B
              (Default|CallNextPenMovetoIdle))))))
    (:NewEnumerator1
      (Timeline|Timeline_1 PlayFromStart))
    (:NewEnumerator2
      (Timeline|Timeline PlayFromStart))))

(fn ConstructionScript)