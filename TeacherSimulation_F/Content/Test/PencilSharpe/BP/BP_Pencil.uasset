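; BP_Pencil is a pencil actor for a hold-to-sharpen minigame, using per-pencil timelines to move into play and back.
; Holding TestHoldBtn moves it into the sharpener, then shrinks its Z scale with looping camera shakes and sound.
; Release grades the scale band, setting tip mesh and morph target and reporting progress.
; Sharp or over-sharpened pencils return, then FlipFlop disables input and calls the next pencil.
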(event Custom|CustomEvent
  (Camera|PlayWorldCameraShake "/Game/inputs/pencil_and_PencilCameraShake.pencil_and_PencilCameraShake_C" (Transformation|GetActorLocation (Variables|Default|Getbp_cameraRef)) 0.0 5e+02))

(event Custom|Progress
  (params (sharpe :type Boolean))
  ;[0 0 0 0.5] Medium Sharpe Pencil
)

(event Input|EnhancedActionEvents|EnhancedInputActionTestHoldBtn
  (params (ActionValue :type Boolean) (ElapsedSeconds :type Float%20%28double-precision%29) (TriggeredSeconds :type Float%20%28double-precision%29) (InputAction :type Input%20Action%20Object%20Reference :default "/Game/inputs/TestHoldBtn.TestHoldBtn"))
  (bind _returnvalue (Transformation|GetActorScale3D))
  (:Started
    (Variables|Default|SetReady true)
    (if (Variables|Default|GetCanSharpe)
      (bind (_direction _newtrack_0 _newtrack_2) (Timeline|Timeline Play)
        (:Update
          (Transformation|SetActorLocationAndRotation _newtrack_0 (Math|Rotator|MakeRotator 0.0 (.y _newtrack_2) (.z _newtrack_2))))
        (:Finished
          (if (and (Variables|Default|GetReady) (== (.yaw (Transformation|GetActorRotation)) 12.0))
            (bind _returnvalue_2 (Audio|SpawnSound2D "/Game/Assets/sounds/sharpner.sharpner" 1.0 1.0 0.0 0))
            (Variables|Default|SetsharpnerSound _returnvalue_2)
            (Utilities|FlowControl|Sequence
              (:then_0
                (Camera|PlayWorldCameraShake "/Game/inputs/pencil_and_PencilCameraShake.pencil_and_PencilCameraShake_C" (Transformation|GetActorLocation (Variables|Default|Getbp_cameraRef)) 0.0 5e+02)
                (bind _returnvalue_3 (Utilities|Time|SetTimerbyEvent (delegate Custom|CustomEvent) 0.5 true))
                (Variables|Default|SettimerEvent _returnvalue_3))
              (:then_1
                (bind (_direction_2 _newtrack_0_2 _newtrack_2_2) (Timeline|Timeline_1 Play)
                  (:Update
                    (Transformation|SetActorScale3D (Math|Vector|MakeVector 1.0 1.0 _newtrack_0_2))
                    (Transformation|SetActorLocation _newtrack_2_2 false false))))))))))
  (:Canceled
    (Variables|Default|SetReady false :!label _label)
    (Utilities|FlowControl|Sequence
      (:then_0
        (bind _sharpnersound (Variables|Default|GetsharpnerSound)
          (:then
            (Audio|Components|Audio|Stop _sharpnersound))
          (:else
            _))
        (Utilities|FlowControl|Sequence
          (:then_0
            (Timeline|Timeline_1 Stop))
          (:then_1
            (Utilities|Time|ClearandInvalidateTimerbyHandle (Variables|Default|GettimerEvent)))))
      (:then_1
        (Timeline|Timeline Reverse))
      (:then_2
        ;[0 0 0 0.5] Not Sharpe Pencil
        (if (and (<= (.z _returnvalue) 0.99) (> (.z _returnvalue) 0.95))
          (Development|PrintString "not Sharpe")
          (Variables|Default|SetReady true)
          (Components|StaticMesh|SetStaticMesh (Variables|Default|Gettip) 0)
          (Components|SkeletalMesh|SetMorphTarget (Variables|Default|Getpencil__1_) "pCylinder3" 0.2 true)
          (else
            ;[0 0 0 0.5] Medium Sharpe Pencil
            (if (and (<= (.z _returnvalue) 0.95) (> (.z _returnvalue) 0.85))
              (Development|PrintString "Medium Sharpe" :!label _label_2)
              (Default|CallPencilProgress true)
              (Variables|Default|SetReady true)
              (Components|StaticMesh|SetStaticMesh (Variables|Default|Gettip) "/Game/Assets/PencilAndSharpner/T_05.T_05")
              (Components|SkeletalMesh|SetMorphTarget (Variables|Default|Getpencil__1_) "pCylinder3" 0.5 true)
              (elif (and (<= (.z _returnvalue) 0.7) (> (.z _returnvalue) 0.65))
                (goto _label_2)
                (else
                  ;[0 0 0 0.5] Sharpe Pencil
                  (if (and (<= (.z _returnvalue) 0.85) (> (.z _returnvalue) 0.7))
                    (Default|CallPencilProgress false :!label _label_3)
                    (Development|PrintString "Sharpe")
                    (Components|StaticMesh|SetStaticMesh (Variables|Default|Gettip) "/Game/Assets/PencilAndSharpner/T_1.T_1")
                    (Components|SkeletalMesh|SetMorphTarget (Variables|Default|Getpencil__1_) "pCylinder3" 1.0 true)
                    (Audio|PlaySound2D "/Game/Assets/sounds/pencilsharped.pencilsharped" 1.0 1.0 0.0 0 0)
                    (Variables|Default|SetReady false :!label _label_4)
                    (Variables|Default|SetCanSharpe false)
                    (Utilities|FlowControl|Delay 1.0)
                    (Utilities|FlowControl|DoOnce false
                      (:Completed
                        (switch Utilities|FlowControl|Switch|SwitchonE_PencilNo (stale EventMoveobjecttoIdlePos NewParam)
                          (:NewEnumerator0
                            (bind (_direction_3 _newtrack_2_3 _newtrack_0_3) (Timeline|Timeline_0 ReverseFromEnd)
                              (:Update
                                (Transformation|SetActorLocationAndRotation _newtrack_2_3 (Math|Rotator|MakeRotator 0.0 (.y _newtrack_0_3) (.z _newtrack_0_3))))
                              (:Finished
                                (Input|EnableInput (Game|GetPlayerController 0) :!label _label_5)
                                (Utilities|FlowControl|FlipFlop
                                  (:B
                                    (Input|DisableInput (Game|GetPlayerController 0))
                                    (Default|CallNextPencilMovetoIdle))))))
                          (:NewEnumerator1
                            (bind (_direction_4 _newtrack_2_4 _newtrack_0_4) (Timeline|Timeline_4 ReverseFromEnd)
                              (:Update
                                (Transformation|SetActorLocationAndRotation _newtrack_2_4 (Math|Rotator|MakeRotator 0.0 (.y _newtrack_0_4) (.z _newtrack_0_4))))
                              (:Finished
                                (goto _label_5))))
                          (:NewEnumerator2
                            (bind (_direction_5 _newtrack_2_5 _newtrack_0_5) (Timeline|Timeline_2 ReverseFromEnd)
                              (:Update
                                (Transformation|SetActorLocationAndRotation _newtrack_2_5 (Math|Rotator|MakeRotator 0.0 (.y _newtrack_0_5) (.z _newtrack_0_5))))
                              (:Finished
                                (goto _label_5)))))))
                    (elif (and (<= (.z _returnvalue) 0.65) (> (.z _returnvalue) 0.4))
                      (goto _label_3)
                      (elif (<= (.z _returnvalue) 0.4)
                        (Default|CallPencilProgress true)
                        (Components|StaticMesh|SetStaticMesh (Variables|Default|Gettip) "/Game/Assets/PencilAndSharpner/T_05.T_05")
                        (Components|SkeletalMesh|SetMorphTarget (Variables|Default|Getpencil__1_) "pCylinder3" 0.5 true)
                        (goto _label_4))))))))))))
  (:Completed
    (goto _label)))

(event EventMoveobjecttoIdlePos
  (params (NewParam :type E_PencilNo%20Enum :default "NewEnumerator0"))
  (Input|EnableInput (Game|GetPlayerController 0))
  (Variables|Default|SetStartingLocation (Transformation|GetActorLocation))
  (Utilities|FlowControl|Delay 0.2)
  (bind _returnvalue (Actor|GetActorOfClass "/Game/Test/InkPot/BluePrint/BP_Camera_02.BP_Camera_02_C"))
  (Variables|Default|Setbp_cameraRef _returnvalue)
  (switch Utilities|FlowControl|Switch|SwitchonE_PencilNo NewParam
    (:NewEnumerator0
      (bind (_direction _newtrack_2 _newtrack_0) (Timeline|Timeline_0 PlayFromStart)
        (:Update
          (Transformation|SetActorLocationAndRotation _newtrack_2 (Math|Rotator|MakeRotator 0.0 (.y _newtrack_0) (.z _newtrack_0))))
        (:Finished
          (Input|EnableInput (Game|GetPlayerController 0) :!label _label)
          (Utilities|FlowControl|FlipFlop
            (:B
              (Input|DisableInput (Game|GetPlayerController 0))
              (Default|CallNextPencilMovetoIdle))))))
    (:NewEnumerator1
      (bind (_direction_2 _newtrack_2_2 _newtrack_0_2) (Timeline|Timeline_4 PlayFromStart)
        (:Update
          (Transformation|SetActorLocationAndRotation _newtrack_2_2 (Math|Rotator|MakeRotator 0.0 (.y _newtrack_0_2) (.z _newtrack_0_2))))
        (:Finished
          (goto _label))))
    (:NewEnumerator2
      (bind (_direction_3 _newtrack_2_3 _newtrack_0_3) (Timeline|Timeline_2 PlayFromStart)
        (:Update
          (Transformation|SetActorLocationAndRotation _newtrack_2_3 (Math|Rotator|MakeRotator 0.0 (.y _newtrack_0_3) (.z _newtrack_0_3))))
        (:Finished
          (goto _label))))))

(fn ConstructionScript)