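; Level 3 teacher Blueprint that walks to a chosen student and turns using timelines.
; On BeginPlay it caches all StudentBP_lvl3 actors, then MoveToTheStudent slides the root to that student's X plus an offset on a fixed Y line.
; Timelines drive yaw for the first two students, and the second also changes the offset when finished.
; TeacherBackToCurrentPosition alternately reverses those timelines through a FlipFlop, undoing only rotation.
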(event Custom|MoveToTheStudent
  (params (studentIndex :type Integer))
  (Variables|Default|SetCurrentStudent%20Index studentIndex)
  (Utilities|FlowControl|Delay 0.2)
  (Components|MoveComponentTo (Variables|Default|GetDefaultSceneRoot) (Math|Vector|MakeVector (+ (.x (Transformation|GetWorldLocation (Variables|/Game/Blueprints/Student/StudentBP.StudentBP_C|GetDefaultSceneRoot (Utilities|Array|Get(acopy) (Variables|Default|GetOut%20Actors) studentIndex)))) (Variables|Default|GetoffsetStd)) 1424.950977 0.0) "0, 0, 0" false false 3.0 false)
  (switch int (Variables|Default|GetCurrentStudent%20Index)
    (:0
      (bind _newtrack_0 (Timeline|Timeline_0_0 PlayFromStart)
        (:Update
          (Transformation|SetActorRotation (Math|Rotator|MakeRotator 0.0 0.0 _newtrack_0)))))
    (:1
      (bind _newtrack_0_2 (Timeline|Timeline_1 PlayFromStart)
        (:Update
          (Transformation|SetActorRotation (Math|Rotator|MakeRotator 0.0 0.0 _newtrack_0_2)))
        (:Finished
          (Variables|Default|SetoffsetStd -3e+02))))))

(event Custom|TeacherBackToCurrentPosition
  (if (< (Variables|Default|GetCurrentStudent%20Index) 2)
    (Utilities|FlowControl|FlipFlop
      (:A
        (bind _newtrack_0 (Timeline|Timeline_0_0 ReverseFromEnd)
          (:Update
            (Transformation|SetActorRotation (Math|Rotator|MakeRotator 0.0 0.0 _newtrack_0)))))
      (:B
        (bind _newtrack_0_2 (Timeline|Timeline_1 ReverseFromEnd)
          (:Update
            (Transformation|SetActorRotation (Math|Rotator|MakeRotator 0.0 0.0 _newtrack_0_2)))
          (:Finished
            (Variables|Default|SetoffsetStd -3e+02)))))))

(event EventBeginPlay
  (|CallParentFunction)
  (bind _outactors (Actor|GetAllActorsOfClass "/Game/Blueprints/Student/StudentBP_lvl3.StudentBP_lvl3_C"))
  (Variables|Default|SetOut%20Actors _outactors))

(fn ConstructionScript
  (|CallParentFunction))