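; Teacher camera actor that plays a stand-up move and shifts focus between students, adding the teacher input mapping context on level03.
; StandAnim drives the root's height with a timeline, then saves the final location as the standing position.
; Focus events use timed MoveComponentTo calls to glide the root to an offset from a student or turn only the camera toward a target.
; Unfocus glides the root back to the saved position.
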(event Custom|focusOnStudent
  (params (NewParam :type Pawn%20Object%20Reference))
  ;[0 0 0 0.5] Focus/Unfocus on a student
  (Components|MoveComponentTo (Variables|Default|GetDefaultSceneRoot) (- (Transformation|GetActorLocation NewParam) "-500.000000,0.000000,-50.000000") "0.000000,180.000000,0.000000" false false 2.0 false))

(event Custom|StandAnim
  (bind _defaultsceneroot (Variables|Default|GetDefaultSceneRoot))
  (bind _returnvalue (Transformation|GetWorldLocation _defaultsceneroot))
  ;[0 0 0 0.5] CameraStandAnimation
  (bind _newtrack_0 (Timeline|Timeline PlayFromStart)
    (:Update
      (Transformation|SetWorldLocation _defaultsceneroot (Math|Vector|MakeVector (.x _returnvalue) (.y _returnvalue) _newtrack_0) false false))
    (:Finished
      (CallFunction|SetPlayerStartPos))))

(event Custom|UnFocusStudents
  ;[0 0 0 0.5] Focus/Unfocus on a student
  (Components|MoveComponentTo (Variables|Default|GetDefaultSceneRoot) (Variables|Default|GetCameraStandingPostion) "0.000000,180.000000,0.000000" false false 2.0 false))

(event Custom|OnlyFocusOnTarget
  (params (NewParam :type Pawn%20Object%20Reference))
  (bind _returnvalue (Transformation|GetActorLocation NewParam))
  (bind _returnvalue_2 (Game|GetPlayerController 0))
  (bind _camera (Variables|Default|GetCamera))
  (bind _returnvalue_3 (Transformation|GetWorldLocation _camera))
  (bind _playercameramanager (Variables|/Script/Engine.PlayerController|GetPlayerCameraManager _returnvalue_2))
  (bind _returnvalue_4 (Math|Rotator|FindLookatRotation _returnvalue_3 _returnvalue))
  (bind _returnvalue_5 (Transformation|GetActorRotation _playercameramanager))
  (Components|MoveComponentTo (Variables|Default|GetCamera) "0, 0, 0" (Math|Rotator|MakeRotator (- (.roll _returnvalue_4) (.roll _returnvalue_5)) (- (.pitch _returnvalue_4) (.pitch _returnvalue_5)) (- (.yaw _returnvalue_4) (.yaw _returnvalue_5))) false false 1.0 false))

(event EventBeginPlay
  ;[0 0 0 0.5] AddAnimationRef
  (bind _returnvalue (Game|GetCurrentLevelName true))
  (if (Utilities|Enum|Equal(Enum) _returnvalue "level03")
    (Input|AddMappingContext (PlayerController|LocalPlayerSubsystems|GetEnhancedInputLocalPlayerSubsystem (Game|GetPlayerController 0)) "/Game/inputs/IAM_Teacher.IAM_Teacher" 0 "(bIgnoreAllPressedKeysUntilRelease=True,bForceImmediately=False,bNotifyUserSettings=False)")))

(fn ConstructionScript)

(fn SetPlayerStartPos
  (Variables|Default|SetCameraStandingPostion (Transformation|GetWorldLocation (Variables|Default|GetDefaultSceneRoot))))