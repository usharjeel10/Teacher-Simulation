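; Student actor for a diagram-matching game that stands in a line, steps forward and reacts happily or sadly before leaving.
; MoveStdForward switches StudentAnimation states around a timed move, and the first student then calls CallUpdateNextDiagram.
; SetJoyAnimation plays a victory or defeat montage, then slides the actor sideways, destroys it and calls CallUpdateNextDiagram.
; The Die event is an empty stub.
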(event Custom|SetJoyAnimation
  (params (IsHappy :type Boolean))
  (if IsHappy
    (Animation|Montage|PlayMontage (Variables|Default|Getstd) "/Game/Assets/MixamoAssets/MixamoAnimations/VictoryIdle_1__UE_Montage.VictoryIdle_1__UE_Montage"
      (:OnCompleted
        _))
    (else
      (Animation|Montage|PlayMontage (Variables|Default|Getstd) "/Game/Assets/MixamoAssets/MixamoAnimations/Defeat_1__UE_Montage.Defeat_1__UE_Montage"
        (:OnCompleted
          _))))
  (Components|MoveComponentTo (Variables|Default|GetDefaultSceneRoot) (+ (Transformation|GetActorLocation) "0.000000,-500.000000,0.000000") "0.000000,-90.000000,0.000000" false false 0.7 false)
  (Actor|DestroyActor)
  (Default|CallUpdateNextDiagram true))

(event Custom|MoveStdForward
  (Default|PlayState (Variables|Default|GetStd_AnimRef) "NewEnumerator5")
  (Components|MoveComponentTo (Variables|Default|GetDefaultSceneRoot) (+ (Transformation|GetActorLocation) "100.000000,0.000000,0.000000") "0.000000,-90.000000,0.000000" false false 1.0 false)
  (Default|PlayState (Variables|Default|GetStd_AnimRef) "NewEnumerator6")
  (if (Variables|Default|GetStudentAtFirst)
    (Default|CallUpdateNextDiagram false)))

(event Custom|Die
  (params (CanDestroy :type Boolean)))

(event EventBeginPlay
  (bind _asstudent_animation (Utilities|Casting|CastToStudentAnimation (Components|SkeletalMesh|GetAnimInstance (Variables|Default|Getstd))))
  (bind _output_get (Variables|Default|SetStd_AnimRef _asstudent_animation))
  (Default|PlayState _output_get "NewEnumerator6"))

(fn ConstructionScript)