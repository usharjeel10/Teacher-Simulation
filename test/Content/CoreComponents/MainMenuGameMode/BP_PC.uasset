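; Main menu Blueprint, apparently the player controller, that shows the main menu and drives a sliding scroll menu.
; BeginPlay creates both widgets, displays WBP_MainMenu and enables the mouse cursor; CreateMenuWidget later adds the stored Menu to the viewport.
; NextMove and BackMove select a step by index, playing or reversing timelines that animate the Menu's ScrollBox offset.
; A DoOnce, reset by the second slide, guards reversing the first.
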(event Custom|NextMove
  (params (NewParam :type Integer))
  ;[0.15 0.15 0.15 0.5] sliding Menu/TeacherJobs
  (switch int NewParam
    (:0
      (bind _slidetimeline (Timeline|Timeline PlayFromStart)
        (:Update
          (Class|ScrollBox|SetScrollOffset (Variables|/Game/UserWidget/Menu.Menu_C|GetScrollBox_75 (Variables|Default|GetMenu)) _slidetimeline))))
    (:1
      (bind _slidetimeline_2 (Timeline|Timeline_0 PlayFromStart)
        (:Update
          (Class|ScrollBox|SetScrollOffset (Variables|/Game/UserWidget/Menu.Menu_C|GetScrollBox_75 (Variables|Default|GetMenu)) _slidetimeline_2)
          (Utilities|FlowControl|DoOnce false) ; enters at Reset
        )))))

(event Custom|BackMove
  (params (NewParam :type Integer))
  ;[0.15 0.15 0.15 0.5] sliding Menu/TeacherJobs
  (switch int NewParam
    (:0
      (Utilities|FlowControl|DoOnce false :!label _label
        (:Completed
          (bind _slidetimeline (Timeline|Timeline ReverseFromEnd)
            (:Update
              (Class|ScrollBox|SetScrollOffset (Variables|/Game/UserWidget/Menu.Menu_C|GetScrollBox_75 (Variables|Default|GetMenu)) _slidetimeline))))))
    (:1
      (bind _slidetimeline_2 (Timeline|Timeline_0 ReverseFromEnd)
        (:Update
          (Class|ScrollBox|SetScrollOffset (Variables|/Game/UserWidget/Menu.Menu_C|GetScrollBox_75 (Variables|Default|GetMenu)) _slidetimeline_2)
          (goto _label Reset))))))

(event EventBeginPlay
  ;[0 0 0 0.5] displayWidget
  (bind _returnvalue (UserInterface|CreateWidget "/Game/UserWidget/Menu.Menu_C"))
  (Variables|Default|SetMenu _returnvalue)
  (bind _returnvalue_2 (UserInterface|CreateWidget "/Game/UserWidget/WBP_MainMenu.WBP_MainMenu_C"))
  (UserInterface|Viewport|AddtoViewport _returnvalue_2 0)
  (Variables|/Script/Engine.PlayerController|SetbShowMouseCursor (Game|GetPlayerController 0) true))

(fn ConstructionScript)

(fn CreateMenuWidget
  (UserInterface|Viewport|AddtoViewport (Variables|Default|GetMenu) 0))