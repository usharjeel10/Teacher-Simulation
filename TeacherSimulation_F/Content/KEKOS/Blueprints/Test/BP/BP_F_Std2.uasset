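; Female student character Blueprint for a queue of students who react happily, sadly or to being sprayed, then leave.
; Its construction script fills modular mesh and material variables from a data table row picked by uniform index and removes the dirt decal on clean students.
; Events drive the animation instance, step the student forward, or play a reaction montage, slide it out, advance the next diagram and destroy it.
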(event Custom|SetJoyAnimation
  (params (IsHappy :type E_Haal_StudentPunishmentState%20Enum :default "NewEnumerator1") (ISLastStd :type Boolean) (MoveTheStudentOutOfTheView :type Vector))
  (switch Utilities|FlowControl|Switch|SwitchonE_Haal_StudentPunishmentState IsHappy
    (:NewEnumerator1
      (Variables|Default|SetMoveTheStudentOutOfTheView MoveTheStudentOutOfTheView)
      (Animation|Montage|PlayMontage (Variables|Default|GetHead) "/Game/Mixamo/Animation/F_Victory_Idle_Montage.F_Victory_Idle_Montage"
        (:OnCompleted
          _)))
    (:NewEnumerator0
      (Variables|Default|SetMoveTheStudentOutOfTheView MoveTheStudentOutOfTheView)
      (Animation|Montage|PlayMontage (Variables|Default|GetHead) "/Game/Mixamo/Animation/F_Defeated_Idle_Montage.F_Defeated_Idle_Montage"
        (:OnCompleted
          _)))
    (:NewEnumerator2
      (Variables|Default|SetMoveTheStudentOutOfTheView MoveTheStudentOutOfTheView)
      (Rendering|SetVisibility (Variables|Default|GetScene) true true)
      (Components|MoveComponentTo (Variables|Default|GetScene) "21.000000,10.000000,-56.000000" "106.000000,30.000000,-180.000000" true false 0.8 false)
      (Animation|Montage|PlayMontage (Variables|Default|GetHead) "/Game/Mixamo/Animation/F_SprayOnStd_Anim_Montage.F_SprayOnStd_Anim_Montage"
        (:OnCompleted
          (Rendering|SetVisibility (Variables|Default|GetScene) false true)))))
  (if ISLastStd
    (Variables|Default|SetMoveTheStudentOutOfTheView "500.000000,0.000000,0.000000"))
  (Components|MoveComponentTo (Variables|Default|GetHead) (+ (Variables|/Script/Engine.SceneComponent|GetRelativeLocation (Variables|Default|GetHead)) (Variables|Default|GetMoveTheStudentOutOfTheView)) "0.000000,-90.000000,0.000000" false false 0.7 false)
  (Default|CallUpdateNextDiagram true)
  (Actor|DestroyActor))

(event Custom|MoveStdForward
  (Default|PlayState (Variables|Default|GetF%20Student%20Animation) "NewEnumerator5")
  (Components|MoveComponentTo (Variables|Default|GetCapsule) (+ (Transformation|GetActorLocation) "100.000000,0.000000,0.000000") "0.000000,-90.000000,0.000000" false false 1.0 false)
  (Default|PlayState (Variables|Default|GetF%20Student%20Animation) "NewEnumerator6")
  (if (Variables|Default|GetStudent%20at%20First)
    (Default|CallUpdateNextDiagram false)))

(event Custom|Die
  (params (CanDestroy :type Boolean)))

(event Custom|RotateStudentToTeacher
  (params (Target%20Relative%20Rotation%20Z%20%28Yaw%29 :type Float%20%28single-precision%29))
  (Animation|Montage|PlayMontage (Variables|Default|GetHead) "/Game/Mixamo/Animation/F_SprayOnStd_Anim_Montage.F_SprayOnStd_Anim_Montage"
    (:then
      (Components|MoveComponentTo (Variables|Default|GetHead) (Variables|/Script/Engine.SceneComponent|GetRelativeLocation (Variables|Default|GetHead)) (Math|Rotator|MakeRotator 0.0 0.0 Target%20Relative%20Rotation%20Z%20%28Yaw%29) false false 0.4 false))))

(event EventBeginPlay
  (bind _asf_student_animation (Utilities|Casting|CastToF_StudentAnimation (Components|SkeletalMesh|GetAnimInstance (Variables|Default|GetHead))))
  (bind _output_get (Variables|Default|SetF%20Student%20Animation _asf_student_animation))
  (Default|PlayState _output_get "NewEnumerator6"))

(fn ConstructionScript
  (if (Variables|Default|Get?IsStudentDirty)
    _
    (else
      (Components|DestroyComponent (Variables|Default|GetDirt_Decal))))
  (Variables|Default|SetCurrentStdUniformIndx (Utilities|Array|Get(acopy) (Variables|Default|GetRandomStudentWuniform) (Variables|Default|GetCurrentStdUniformIndx)))
  (|CallParentFunction)
  (Rendering|SetVisibility (Variables|Default|GetScene) false true)
  (bind _returnvalue (Utilities|GetDataTableRow "/Game/Blueprints/structure/STdUniform/STD_DATA_TABLE.STD_DATA_TABLE" (Utilities|String|StringToName (Utilities|String|ToString(Integer) (Variables|Default|GetCurrentStdUniformIndx))))
    (:then
      (Variables|Default|SetSkinMaterial (.skinColour (Utilities|Struct|BreakStd_Cloths _returnvalue)))
      (Variables|Default|SetTorsoMesh (.TorsoMesh (Utilities|Struct|BreakStd_Cloths _returnvalue)))
      (Variables|Default|SetTorsoMaterial (.TorsoMaterialArray (Utilities|Struct|BreakStd_Cloths _returnvalue)))
      (Variables|Default|SetLegsMesh (.LegMesh (Utilities|Struct|BreakStd_Cloths _returnvalue)))
      (Variables|Default|SetLegsMaterial (.LegMaterialArray (Utilities|Struct|BreakStd_Cloths _returnvalue)))
      (Variables|Default|SetHandsMesh (.HandMesh (Utilities|Struct|BreakStd_Cloths _returnvalue)))
      (Variables|Default|SetHandsMaterial (.HandMaterial (Utilities|Struct|BreakStd_Cloths _returnvalue)))
      (Variables|Default|SetFeetsMesh (.FeetMesh (Utilities|Struct|BreakStd_Cloths _returnvalue)))
      (Variables|Default|SetFeetsMaterial (.FeetMaterial (Utilities|Struct|BreakStd_Cloths _returnvalue)))
      (Variables|Default|SetFullTorsoMesh (.FullTorsoMesh (Utilities|Struct|BreakStd_Cloths _returnvalue)))
      (Variables|Default|SetFullTorsoMaterial (.FullTorsoMaterialArray (Utilities|Struct|BreakStd_Cloths _returnvalue)))
      (Variables|Default|SetTorsoPropMesh (.TorsoPropMesh (Utilities|Struct|BreakStd_Cloths _returnvalue)))
      (Variables|Default|SetTorsoPropMaterial (.TorsoPropMaterialArray (Utilities|Struct|BreakStd_Cloths _returnvalue)))
      (Variables|Default|SetCapMesh (.capMesh (Utilities|Struct|BreakStd_Cloths _returnvalue)))
      (Variables|Default|SetCapMaterial (.CapMaterial (Utilities|Struct|BreakStd_Cloths _returnvalue)))
      (Variables|Default|SetGlassesMesh (.GlassesMesh (Utilities|Struct|BreakStd_Cloths _returnvalue)))
      (Variables|Default|SetGlassesMaterial (.GlassesMaterial (Utilities|Struct|BreakStd_Cloths _returnvalue)))
      (Variables|Default|SetHairMesh (.HairMesh (Utilities|Struct|BreakStd_Cloths _returnvalue)))
      (Variables|Default|SetHairColor (.HairColor (Utilities|Struct|BreakStd_Cloths _returnvalue)))
      (Variables|Default|SetEyebrowsMesh (.EyeBrowMesh (Utilities|Struct|BreakStd_Cloths _returnvalue)))
      (Variables|Default|SetEyebrowsColor (.EyeBrowColor (Utilities|Struct|BreakStd_Cloths _returnvalue))))))