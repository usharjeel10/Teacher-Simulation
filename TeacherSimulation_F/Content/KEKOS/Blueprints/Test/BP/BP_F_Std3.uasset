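; BP_F_Std3 is a student character Blueprint that can raise and lower its hand.
; On BeginPlay it caches the Head mesh's F_StudentAnimation instance and starts its default state.
; HandRaise shows the Widget component and switches the animation state, while HandsDown hides the widget and restores the default.
; The construction script runs the parent's logic, then hides the widget.
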(event Custom|HandsDown
  (Development|SetHiddeninGame (Variables|Default|GetWidget) true false)
  (Default|PlayState (Variables|Default|GetF%20Student%20Animation) "NewEnumerator0"))

(event Custom|HandRaise
  (Development|SetHiddeninGame (Variables|Default|GetWidget) false false)
  (Default|PlayState (Variables|Default|GetF%20Student%20Animation) "NewEnumerator15"))

(event EventBeginPlay
  (bind _asf_student_animation (Utilities|Casting|CastToF_StudentAnimation (Components|SkeletalMesh|GetAnimInstance (Variables|Default|GetHead))))
  (bind _output_get (Variables|Default|SetF%20Student%20Animation _asf_student_animation))
  (Default|PlayState _output_get "NewEnumerator0"))

(fn ConstructionScript
  (|CallParentFunction)
  (Development|SetHiddeninGame (Variables|Default|GetWidget) true false))