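; Teacher player Blueprint for Level 02, where the player looks around and catches a cheating student.
; Touch drags drive controller yaw and pitch, within camera view limits set at BeginPlay.
; Pressing Interact over the student supplied by GetCheatingStd starts an FOV timeline, reversed on cancel.
; An ongoing hold accumulates time and, after two seconds, only prints a caught message.
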(event Custom|Get%20Cheating%20Std
  (params (NewParam :type Pawn%20Object%20Reference))
  ;[0 0 0 0.5] CaughtStudentOnCheating
  (Variables|Default|SetcheatingStd1 NewParam))

(event Input|EnhancedActionEvents|EnhancedInputActionIA_Interact
  (params (ActionValue :type Boolean) (ElapsedSeconds :type Float%20%28double-precision%29) (TriggeredSeconds :type Float%20%28double-precision%29) (InputAction :type Input%20Action%20Object%20Reference :default "/Game/inputs/IA_Interact.IA_Interact"))
  (bind _returnvalue (Game|GetPlayerController 0))
  (bind (_hitresult _returnvalue_2) (Game|Player|GetHitResultUnderCursorbyChannel _returnvalue "TraceTypeQuery2" true))
  ;[0 0 0 0.5] CaughtStudentOnCheating
  (:Started
    (if (and _returnvalue_2 (== (.HitActor (Collision|BreakHitResult _hitresult)) (Variables|Default|GetcheatingStd1)))
      (Variables|Default|SetcanZoom true)
      (bind _newtrack_0 (Timeline|setFV PlayFromStart)
        (:Update
          (Camera|SetFieldOfView (Variables|Default|GetCamera) _newtrack_0)))))
  (:Ongoing
    (if (Variables|Default|GetcanZoom)
      (Variables|Default|SetNewVar (+ (Utilities|Time|GetWorldDeltaSeconds) (Variables|Default|GetNewVar)))
      (if (>= (Variables|Default|GetNewVar) 2.0)
        (Development|PrintString "student caught")
        (Variables|Default|SetNewVar 0.0))))
  (:Canceled
    (Variables|Default|SetNewVar 0.0)
    (Variables|Default|SetcanZoom false)
    (Timeline|setFV Reverse)))

(event EventBeginPlay
  (bind _returnvalue (Game|GetPlayerCameraManager 0))
  (|CallParentFunction)
  ;[0 0 0 0.5] SwipeInputs
  (CallFunction|SetPlayerStartPos)
  (Variables|/Script/Engine.PlayerCameraManager|SetViewYawMax _returnvalue -1.4e+02)
  (Variables|/Script/Engine.PlayerCameraManager|SetViewYawMin _returnvalue -2.2e+02)
  (Variables|/Script/Engine.PlayerCameraManager|SetViewPitchMax _returnvalue 25.0)
  (Variables|/Script/Engine.PlayerCameraManager|SetViewPitchMin _returnvalue -25.0))

(event Input|TouchEvents|InputTouch
  (params (Location :type Vector) (FingerIndex :type ETouchIndex%20Enum))
  (bind _returnvalue (Math|Vector2D|MakeVector2D (.x Location) (.y Location)))
  (bind _looksensitivity (Variables|Default|GetlookSensitivity))
  ;[0 0 0 0.5] SwipeInputs
  (:Pressed
    (Variables|Default|SetTouchStartPos _returnvalue))
  (:Moved
    (bind _output_get (Variables|Default|SetTouchEndPos _returnvalue))
    (Pawn|Input|AddControllerYawInput (* (.x (- _output_get (Variables|Default|GetTouchStartPos))) _looksensitivity))
    (Pawn|Input|AddControllerPitchInput (* (.y (- _output_get (Variables|Default|GetTouchStartPos))) _looksensitivity))
    (Variables|Default|SetTouchStartPos (Variables|Default|GetTouchEndPos))))

(fn ConstructionScript
  (|CallParentFunction))