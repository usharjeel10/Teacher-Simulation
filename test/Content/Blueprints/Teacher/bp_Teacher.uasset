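; Teacher Blueprint that handles the teacher's stand-up animation and camera moves for focusing on students.
; BeginPlay caches the TeacherAnimation instance and adds the teacher input mapping context only in level02.
; StandAnim plays an animation state while a Timeline drives camera height, then saves the root location as the standing position.
; Focus events use MoveComponentTo to glide the root to an offset from the student, or back to that saved position.
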(event Custom|focusOnStudent
  (params (NewParam :type Pawn%20Object%20Reference))
  ;[0 0 0 0.5] Focus/Unfocus on a student
  (Components|MoveComponentTo (Variables|Default|GetDefaultSceneRoot) (- (Transformation|GetActorLocation NewParam) "-500.000000,0.000000,-50.000000") "0.000000,180.000000,0.000000" false false 2.0 false))

(event Custom|StandAnim
  (bind _camera (Variables|Default|GetCamera))
  (bind _returnvalue (Transformation|GetWorldLocation _camera))
  ;[0 0 0 0.5] CameraStandAnimation
  (Default|PlayState (Variables|Default|GetTeacher%20AnimationRef) "NewEnumerator1")
  (bind _newtrack_0 (Timeline|Timeline PlayFromStart)
    (:Update
      (Transformation|SetWorldLocation _camera (Math|Vector|MakeVector (.x _returnvalue) (.y _returnvalue) _newtrack_0) false false))
    (:Finished
      (CallFunction|SetPlayerStartPos))))

(event Custom|UnFocusStudents
  ;[0 0 0 0.5] Focus/Unfocus on a student
  (Components|MoveComponentTo (Variables|Default|GetDefaultSceneRoot) (Variables|Default|GetCameraStandingPostion) "0.000000,180.000000,0.000000" false false 2.0 false))

(event EventBeginPlay
  ;[0 0 0 0.5] AddAnimationRef
  (bind _asteacher_animation (Utilities|Casting|CastToTeacherAnimation (Components|SkeletalMesh|GetAnimInstance (Variables|Default|GetSkeletalMesh))))
  (Variables|Default|SetTeacher%20AnimationRef _asteacher_animation)
  (bind _returnvalue (Game|GetCurrentLevelName true))
  (if (Utilities|Enum|Equal(Enum) _returnvalue "level02")
    (Input|AddMappingContext (PlayerController|LocalPlayerSubsystems|GetEnhancedInputLocalPlayerSubsystem (Game|GetPlayerController 0)) "/Game/inputs/IAM_Teacher.IAM_Teacher" 0 "(bIgnoreAllPressedKeysUntilRelease=True,bForceImmediately=False,bNotifyUserSettings=False)")))

(fn ConstructionScript)

(fn SetPlayerStartPos
  (Variables|Default|SetCameraStandingPostion (Transformation|GetWorldLocation (Variables|Default|GetDefaultSceneRoot))))