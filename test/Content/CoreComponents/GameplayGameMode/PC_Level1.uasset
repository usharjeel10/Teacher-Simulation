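; PC_Level1 is the player controller for Level 1, a classroom level with students and a whiteboard question.
; On BeginPlay it shows the cursor, adds the level widget, and caches the BP_Camera pawn and a StudentAndCameraInteraction actor.
; Custom events relay focus and unfocus to the camera and answer checks to the current student.
; Another plays the whiteboard focus sequence and sets the board text; resetCameraPos is empty.
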(event Custom|FocusOnWhiteBoardQuestion
  (bind _returnvalue (Sequencer|Player|CreateLevelSequencePlayer "/Game/Sequencer/FocusOnWhiteBoard.FocusOnWhiteBoard"))
  (Sequencer|Player|Play _returnvalue :!class /Script/MovieScene.MovieSceneSequencePlayer)
  (bind _outactors (Actor|GetAllActorsOfClass "/Game/Blueprints/Actors/BP_WhiteBoard.BP_WhiteBoard_C"))
  (Default|SetTextonWhiteBoard (Utilities|Array|Get(acopy) _outactors)))

(event Custom|CheckAnswerTrueORFalse
  (params (?True :type Boolean))
  (Default|StudentChooseAnswer (Variables|Default|GetcurrentStd) ?True))

(event Custom|FoucusOnTarget
  ;[0 0 0 0.5] FocusAndUnfocus On Target
  (Default|FocusonStudent (Variables|Default|GetBp%20Camera_ref) (Variables|Default|GetcurrentStd)))

(event Custom|BackToLocation
  ;[0 0 0 0.5] FocusAndUnfocus On Target
  (Default|UnFocusStudents (Variables|Default|GetBp%20Camera_ref)))

(event Custom|resetCameraPos)

(event Custom|FindStudentAnswer
  (params (true :type Boolean))
  ;[0 0 0 0.5] CheckStudentsAnswer
  (Default|CheckAnswer (Variables|Default|GetcurrentStd) true))

(event EventBeginPlay
  ;[0 0 0 0.5] enableInputs, user widget and get a refference of a teacher class
  (Variables|/Script/Engine.PlayerController|SetbShowMouseCursor self true)
  (bind _returnvalue (UserInterface|CreateWidget "/Game/UserWidget/gamePlayerWBPlevel01.gamePlayerWBPlevel01_C"))
  (bind _output_get (Variables|Default|SetGamePlayWBP_ref _returnvalue))
  (UserInterface|Viewport|AddtoViewport _output_get 0)
  (bind _asbp_camera (Utilities|Casting|CastToBP_Camera (Game|Player|GetPlayerPawn 0)))
  (Variables|Default|SetBp%20Camera_ref _asbp_camera)
  (bind _returnvalue_2 (Actor|GetActorOfClass "/Game/CoreComponents/StudentAndCameraInteraction.StudentAndCameraInteraction_C"))
  (Variables|Default|SetST_ActorRef _returnvalue_2))

(fn ConstructionScript)