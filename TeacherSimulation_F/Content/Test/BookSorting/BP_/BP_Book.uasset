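; BP_Book is a selectable book in a book-sorting test.
; SelectBook alternates through a FlipFlop, applying the arrow material and marking the book selected only if it is on top, or clearing both.
; UnSelectedBook shares the clearing path without toggling the FlipFlop.
; SetState stores the passed state and uses a counter to clear the on-top flag once the counter has reached one.
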(event Custom|SelectBook
  (Utilities|FlowControl|FlipFlop
    (:A
      (if (Variables|Default|Get?OnTop)
        (Rendering|Material|SetMaterial (Variables|Default|GetBook) 0 "/Engine/VREditor/UI/ArrowMaterial.ArrowMaterial")
        (Variables|Default|Set?Selected true)))
    (:B
      (if (Variables|Default|Get?Selected)
        (Rendering|Material|SetMaterial (Variables|Default|GetBook) 0 0)
        (Variables|Default|Set?Selected false)))))

(event Custom|UnSelectedBook
  (if (Variables|Default|Get?Selected)
    (Rendering|Material|SetMaterial (Variables|Default|GetBook) 0 0)
    (Variables|Default|Set?Selected false)))

(event Custom|SetState
  (params (NewParam :type E_BookInCupboard%20Enum :default "NewEnumerator4"))
  (Variables|Default|SetE_BS NewParam)
  (if (>= (Variables|Default|Getcounter) 1)
    (Variables|Default|Set?OnTop false)
    (else
      (Math|Integer|IncrementInt (Variables|Default|Getcounter)))))

(fn ConstructionScript)