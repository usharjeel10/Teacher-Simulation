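; Classroom student pawn for a quiz game that holds one answer from the question data table and reacts to the player's verdict on it.
; It drives the student animation states, arrow and answer-box widgets, with the second answer hardcoded as correct.
; For the whiteboard sequence, a timeline moves the student along a level spline, then AIMoveTo returns them to the start.
; Level completion is only printed; otherwise the student is unfocused for another try.
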(event Custom|studentStateInClassroom
  (params (selectState :type E_Std_Anim_State%20Enum :default "NewEnumerator0"))
  ;[0 0 0 0.5] SetStudentAnimation
  (Default|PlayState (Variables|Default|GetStudent%20AnimationRef) selectState))

(event Custom|findStudentAndDisplayArrow
  (params (NewParam :type Byte) (Tries :type Integer))
  ;[0 0 0 0.5] EnableAnswersBoxONStudents
  (Variables|Default|SetTries Tries)
  (Variables|Default|SetcanStand true)
  (Development|SetHiddeninGame (Variables|Default|GetWidget) false false)
  (Variables|Default|SetE_AnswerIndex (Utilities|Enum|ByteToEnumStudentAnswerIndex NewParam))
  (Utilities|FlowControl|DoOnce false
    (:Completed
      ;[0 0 0 0.5] AddAnswersToStudents
      (Rendering|Components|TextRender|SetText (Variables|/Game/UserWidget/WBP_AnswerBox.WBP_AnswerBox_C|GetTextBlock_250 (stale EventBeginPlay _aswbp_answer_box)) (Utilities|Select :Index (Variables|Default|GetE_AnswerIndex) :NewEnumerator0 (.answer1 (.ans (stale EventBeginPlay _returnvalue_2))) :NewEnumerator1 (.answer2 (.ans (stale EventBeginPlay _returnvalue_2))) :NewEnumerator2 (.answer3 (.ans (stale EventBeginPlay _returnvalue_2))) :NewEnumerator3 (.answer4 (.ans (stale EventBeginPlay _returnvalue_2)))))
      ;[0 0 0 0.5] GetStudentWrongAndTrueAnswer
      (switch Utilities|FlowControl|Switch|SwitchonStudentAnswerIndex (Variables|Default|GetE_AnswerIndex)
        (:NewEnumerator0
          (Variables|Default|SetFalseAnswer true :!label _label))
        (:NewEnumerator1
          (Variables|Default|SetTrueAnswer true))
        (:NewEnumerator2
          (goto _label))
        (:NewEnumerator3
          (goto _label))))))

(event Custom|disable%20Arrow
  ;[0 0 0 0.5] Disable Arrow When Student Stand
  (Development|SetHiddeninGame (Variables|Default|GetWidget) true false))

(event Custom|ShowAnswerBox
  ;[0 0 0 0.5] Show Answers Box
  (Variables|Default|SetcanStand false)
  (Utilities|FlowControl|Delay 2.0)
  (Development|SetHiddeninGame (Variables|Default|GetW_answerBox) false false))

(event Custom|checkAnswer
  (params (True :type Boolean))
  ;[0 0 0 0.5] Check Answer (if true then complete gama. base on the answers play animations and stop the game)............... For Level  01
  (if True
    (if (Variables|Default|GetTrueAnswer)
      (Variables|/Game/CoreComponents/GameplayGameMode/PC_Level1.PC_Level1_C|SetCanUnfocusOnStudent (Variables|Default|GetPC%20Level%201) false)
      (Default|PlayState (Variables|Default|GetStudent%20AnimationRef) "NewEnumerator9")
      (Default|CallOnChoice)
      (Development|PrintString "complete Level/HappyAnimation" true true "(R=0.000000,G=1.000000,B=0.141202,A=1.000000)" 14.0 :!label _label)
      (Utilities|FlowControl|Delay 2.0)
      (Rendering|SetVisibility (Variables|Default|GetW_answerBox) false false)
      (else
        (Default|PlayState (Variables|Default|GetStudent%20AnimationRef) "NewEnumerator9")
        (Default|CallOnBadChoice)
        (Utilities|FlowControl|Delay 2.0 :!label _label_2)
        (Rendering|SetVisibility (Variables|Default|GetW_answerBox) false false)))
    (elif (Variables|Default|GetTrueAnswer)
      (Variables|/Game/CoreComponents/GameplayGameMode/PC_Level1.PC_Level1_C|SetCanUnfocusOnStudent (Variables|Default|GetPC%20Level%201) false)
      (Default|PlayState (Variables|Default|GetStudent%20AnimationRef) "NewEnumerator10")
      (Default|CallOnBadChoice)
      (goto _label)
      (else
        (if (Variables|Default|GetFalseAnswer)
          _
          (else
            _))
        (Default|PlayState (Variables|Default|GetStudent%20AnimationRef) "NewEnumerator10")
        (Default|CallOnChoice)
        (goto _label_2)))))

(event Custom|MoveStudentToWhiteBoard
  ;[0 0 0 0.5] Student Moving to the board Play Animation and Back To the Position .............................. Level 05
  (bind _result (Math|Integer|DecrementInt (Variables|Default|GetTries))
    (:%20%20
      (Variables|Default|SetTries _result)
      (Variables|Default|SetStudentStartingPos (Transformation|GetActorLocation))
      (Utilities|FlowControl|Delay 2.0)
      (Default|PlayState (Variables|Default|GetStudent%20AnimationRef) "NewEnumerator5")
      (bind _newtrack_0 (Timeline|SplineMovement PlayFromStart)
        (:Update
          (Transformation|SetActorLocationAndRotation (.location (Spline|GetTransformatDistanceAlongSpline (Variables|/Game/Blueprints/Actors/Spline.Spline_C|GetSpline (Variables|Default|Getspline)) (Math|Float|Lerp 0.0 (Spline|GetSplineLength (Variables|/Game/Blueprints/Actors/Spline.Spline_C|GetSpline (Variables|Default|Getspline))) _newtrack_0) "World" false)) (.rotation (Spline|GetTransformatDistanceAlongSpline (Variables|/Game/Blueprints/Actors/Spline.Spline_C|GetSpline (Variables|Default|Getspline)) (Math|Float|Lerp 0.0 (Spline|GetSplineLength (Variables|/Game/Blueprints/Actors/Spline.Spline_C|GetSpline (Variables|Default|Getspline))) _newtrack_0) "World" false))))
        (:Finished
          (Default|PlayState (Variables|Default|GetStudent%20AnimationRef) "NewEnumerator6"))))))

(event Custom|StudentChooseAnswer
  (params (TrueAnswer :type Boolean))
  ;[0 0 0 0.5] Student Moving to the board Play Animation and Back To the Position .............................. Level 05
  (Default|PlayState (Variables|Default|GetStudent%20AnimationRef) "NewEnumerator7")
  (Utilities|FlowControl|Delay 4.5)
  (Transformation|SetActorRotation "0.000000,180.000000,0.000000")
  (if TrueAnswer
    (Default|PlayState (Variables|Default|GetStudent%20AnimationRef) "NewEnumerator9")
    (else
      (Default|PlayState (Variables|Default|GetStudent%20AnimationRef) "NewEnumerator10")))
  (Utilities|FlowControl|Delay 5.5)
  (bind _returnvalue (Actor|GetActorOfClass "/Game/Blueprints/Teacher/BP_Camera.BP_Camera_C"))
  (Game|Player|SetViewTargetwithBlend (Game|GetPlayerController 0) _returnvalue 1.0 "VTBlend_Linear" 0.0 false)
  (Default|PlayState (Variables|Default|GetStudent%20AnimationRef) "NewEnumerator5")
  (AI|AIMoveTo self (Variables|Default|GetStudentStartingPos) 0 5.0 false
    (:OnSuccess
      (Transformation|SetActorRotation (Math|Interpolation|RInterpTo "0.000000,180.000000,0.000000" "0, 0, 0" 1.0 1.0))
      (Default|PlayState (Variables|Default|GetStudent%20AnimationRef) "NewEnumerator2")
      (Utilities|FlowControl|Delay 1.0)
      (if TrueAnswer
        (Development|PrintString "LevelComplete!!!!!!!!!!!!!" true true "(R=0.000000,G=0.660000,B=1.000000,A=1.000000)" 1e+01 :!label _label)
        (elif (< (Variables|Default|GetTries) -1)
          (goto _label)
          (else
            (bind _returnvalue_2 (Actor|GetActorOfClass "/Game/CoreComponents/StudentAndCameraInteraction.StudentAndCameraInteraction_C"))
            (Default|UnfocusStudent _returnvalue_2)))))))

(event EventBeginPlay
  ;[0 0 0 0.5] Animation&AnswersRef(DataTable)
  (bind _returnvalue (Actor|GetActorOfClass "/Game/Blueprints/Actors/Spline.Spline_C"))
  (Variables|Default|Setspline _returnvalue)
  (bind _asstudent_animation (Utilities|Casting|CastToStudentAnimation (Components|SkeletalMesh|GetAnimInstance (Variables|Default|GetSM_Student))))
  (Variables|Default|SetStudent%20AnimationRef _asstudent_animation)
  (bind _aswbp_answer_box (Utilities|Casting|CastToWBP_AnswerBox (UserInterface|GetUserWidgetObject (Variables|Default|GetW_answerBox))))
  (bind _aspc_level_1 (Utilities|Casting|CastToPC_Level1 (Game|GetPlayerController 0)))
  (Variables|Default|SetPC%20Level%201 _aspc_level_1)
  ;[0 0 0 0.5] AddAnswersToStudents
  (bind _returnvalue_2 (Utilities|GetDataTableRow "/Game/Blueprints/dataTables/DT_QuestionAnswers.DT_QuestionAnswers" "q1")))

(fn ConstructionScript
  (Development|SetHiddeninGame (Variables|Default|GetWidget) true false)
  (Development|SetHiddeninGame (Variables|Default|GetW_answerBox) true false))

(fn GetSelectStdRef
  (params (NewParam :type Pawn%20Object%20Reference))
  (return self))