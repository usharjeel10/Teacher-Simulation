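; Glass for the volcano scenario that fills with pink or blue liquid, then signals the volcano is full.
; Colour changes spawn a new Liquid layer at the previous one's Scene1 point, grown by timeline scaling, while particles and rotating pour components show pouring.
; A countdown ends filling, calls CallFullTheVolcano and destroys the layers.
; A separate FlipFlop event moves a mesh to open or close the volcano, with smoke on alternate calls.
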(event Custom|StopPinkLiquid
  (params (NewParam :type LiquidState%20Enum :default "NewEnumerator0"))
  (Utilities|FlowControl|Sequence
    (:then_0
      (bind _newtrack_0 (Timeline|Timeline_2 Stop)
        (:Update
          (Transformation|SetWorldScale3D (Variables|/Game/Test/VolcanoScenario/BP/Liquid.Liquid_C|GetScale (Variables|Default|GetCurrentObj)) (Math|Vector|MakeVector 0.25 _newtrack_0 0.25))
          (Variables|Default|SetNewVar (Math|Float|Clamp(Float) (- (Variables|Default|GetNewVar) (Utilities|Time|GetWorldDeltaSeconds)) 0.0 4.0))
          (if (<= (Variables|Default|GetNewVar) 0.0)
            (Variables|Default|Set?CanFill false)
            (Default|CallFulltheVolcano)
            (Utilities|FlowControl|Sequence
              (:then_0
                (Timeline|Timeline_2 Stop))
              (:then_1
                (Utilities|FlowControl|Delay 1.0)
                (for _array_element (Variables|Default|GetLiquidArray)
                  (Actor|DestroyActor _array_element)))
              (:then_2
                (switch Utilities|FlowControl|Switch|SwitchonLiquidState (Variables|Default|GetlS)
                  (:NewEnumerator0
                    (Rendering|SetVisibility (Variables|Default|GetParticleSystem1) false false)
                    (bind _newtrack_1 (Timeline|Timeline_3 Reverse)
                      (:Update
                        (Transformation|SetRelativeRotation (Variables|Default|Getploy1) (Math|Rotator|MakeRotator 0.0 _newtrack_1 1.8e+02) false false))))
                  (:NewEnumerator1
                    (Rendering|SetVisibility (Variables|Default|GetParticleSystem) false false)
                    (bind _newtrack_1_2 (Timeline|Timeline_1 Reverse)
                      (:Update
                        (Transformation|SetRelativeRotation (Variables|Default|Getploy) (Math|Rotator|MakeRotator 0.0 _newtrack_1_2 0.0) false false)))))))))))
    (:then_1
      (Utilities|FlowControl|DoOnce false) ; enters at Reset
    )
    (:then_2
      (switch Utilities|FlowControl|Switch|SwitchonLiquidState NewParam
        (:NewEnumerator0
          (Rendering|SetVisibility (Variables|Default|GetParticleSystem1) false false)
          (Timeline|Timeline_3 Reverse))
        (:NewEnumerator1
          (Rendering|SetVisibility (Variables|Default|GetParticleSystem) false false)
          (Timeline|Timeline_1 Reverse))))))

(event Custom|Open/CloseVolcano
  (params (Cofettee :type Boolean))
  (bind _smokelocation (Variables|Default|GetSmokeLocation))
  (bind _returnvalue (Transformation|GetWorldLocation _smokelocation))
  (Utilities|FlowControl|FlipFlop
    (:A
      (Components|MoveComponentTo (Variables|Default|GetStaticMesh2) "0.000000,900.000000,900.000000" "90.000000,0.000000,180.000000" false false 0.2 false))
    (:B
      (Components|MoveComponentTo (Variables|Default|GetStaticMesh2) "5.000000,210.000000,0.000000" "90.000000,0.000000,180.000000" true false 0.2 false)
      (Utilities|FlowControl|Delay 0.6)
      (if Cofettee
        (Effects|SpawnEmitteratLocation "/Game/Test/VolcanoScenario/BP/Effects/VolcanoSmoke.VolcanoSmoke" _returnvalue)
        (else
          (Effects|SpawnEmitteratLocation "/Game/Test/VolcanoScenario/BP/Effects/VolcanoSmoke.VolcanoSmoke" _returnvalue))))))

(event Custom|AddPinkLiquid
  (params (?IsBlue :type Boolean) (NewParam :type LiquidState%20Enum :default "NewEnumerator0"))
  (if (Variables|Default|Get?CanFill)
    (Utilities|FlowControl|Sequence
      (:then_0
        (Utilities|FlowControl|DoOnce false
          (:Completed
            (if (not (Utilities|Enum|Equal(Enum) NewParam (Variables|Default|GetlS)))
              (Variables|Default|SetlS NewParam)
              (Utilities|FlowControl|Sequence
                (:then_0
                  (bind _returnvalue (Game|SpawnActorfromClass "/Game/Test/VolcanoScenario/BP/Liquid.Liquid_C" (Math|Transform|MakeTransform (Math|Vector|MakeVector (.x (Transformation|GetWorldLocation (Variables|/Game/Test/VolcanoScenario/BP/Liquid.Liquid_C|GetScene1 (Variables|Default|GetCurrentObj)))) (.y (Transformation|GetWorldLocation (Variables|/Game/Test/VolcanoScenario/BP/Liquid.Liquid_C|GetScene1 (Variables|Default|GetCurrentObj)))) (.z (Transformation|GetWorldLocation (Variables|/Game/Test/VolcanoScenario/BP/Liquid.Liquid_C|GetScene1 (Variables|Default|GetCurrentObj))))) "0, 0, 0" "1.000000,0.100000,1.000000") "Undefined" "MultiplyWithRoot" 0 0))
                  (bind _output_get (Variables|Default|SetCurrentObj _returnvalue))
                  (Utilities|Array|Add (Variables|Default|GetLiquidArray) _output_get)
                  (if ?IsBlue
                    (Rendering|Material|SetMaterial (Variables|/Game/Test/VolcanoScenario/BP/Liquid.Liquid_C|GetSM_L01 _output_get) 0 "/Engine/VREditor/UI/ArrowMaterial.ArrowMaterial")
                    (else
                      (Rendering|Material|SetMaterial (Variables|/Game/Test/VolcanoScenario/BP/Liquid.Liquid_C|GetSM_L01 _output_get) 0 "/Game/Assets/SprayBotal/spray-paint/source/banka.banka"))))
                (:then_1
                  (bind _newtrack_0 (Timeline|Timeline_2 SetNewTime)
                    (:Update
                      (Transformation|SetWorldScale3D (Variables|/Game/Test/VolcanoScenario/BP/Liquid.Liquid_C|GetScale (Variables|Default|GetCurrentObj)) (Math|Vector|MakeVector 0.25 _newtrack_0 0.25))
                      (Variables|Default|SetNewVar (Math|Float|Clamp(Float) (- (Variables|Default|GetNewVar) (Utilities|Time|GetWorldDeltaSeconds)) 0.0 4.0))
                      (if (<= (Variables|Default|GetNewVar) 0.0)
                        (Variables|Default|Set?CanFill false)
                        (Default|CallFulltheVolcano)
                        (Utilities|FlowControl|Sequence
                          (:then_0
                            (Timeline|Timeline_2 Stop))
                          (:then_1
                            (Utilities|FlowControl|Delay 1.0)
                            (for _array_element (Variables|Default|GetLiquidArray)
                              (Actor|DestroyActor _array_element)))
                          (:then_2
                            (switch Utilities|FlowControl|Switch|SwitchonLiquidState (Variables|Default|GetlS)
                              (:NewEnumerator0
                                (Rendering|SetVisibility (Variables|Default|GetParticleSystem1) false false)
                                (bind _newtrack_1 (Timeline|Timeline_3 Reverse)
                                  (:Update
                                    (Transformation|SetRelativeRotation (Variables|Default|Getploy1) (Math|Rotator|MakeRotator 0.0 _newtrack_1 1.8e+02) false false))))
                              (:NewEnumerator1
                                (Rendering|SetVisibility (Variables|Default|GetParticleSystem) false false)
                                (bind _newtrack_1_2 (Timeline|Timeline_1 Reverse)
                                  (:Update
                                    (Transformation|SetRelativeRotation (Variables|Default|Getploy) (Math|Rotator|MakeRotator 0.0 _newtrack_1_2 0.0) false false))))))))))))))))
      (:then_1
        (Timeline|Timeline_2 Play))
      (:then_2
        (switch Utilities|FlowControl|Switch|SwitchonLiquidState NewParam
          (:NewEnumerator0
            (Rendering|SetVisibility (Variables|Default|GetParticleSystem1) true false)
            (Timeline|Timeline_3 Play))
          (:NewEnumerator1
            (Rendering|SetVisibility (Variables|Default|GetParticleSystem) true false)
            (Timeline|Timeline_1 Play)))))))

(event EventBeginPlay
  (bind _returnvalue (Game|SpawnActorfromClass "/Game/Test/VolcanoScenario/BP/Liquid.Liquid_C" (Math|Transform|MakeTransform "378.000000,-51.000000,0.000000" "0, 0, 0" "1.000000,0.000000,1.000000") "Undefined" "MultiplyWithRoot" 0 0))
  (Variables|Default|SetCurrentObj _returnvalue))

(fn ConstructionScript
  (Rendering|SetVisibility (Variables|Default|Getploy1) false true))