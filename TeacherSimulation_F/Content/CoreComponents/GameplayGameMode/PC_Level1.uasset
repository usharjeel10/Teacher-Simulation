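; Level 1 player controller for a classroom game where the player judges student answers.
; It creates the gameplay HUD and drives BP_Camera to focus on the current student, whose choice events update good/bad feedback and progress.
; A Level Sequence focuses on the whiteboard question.
; When unfocusing is no longer allowed, it blends to a level camera, removes the HUD and shows the day-complete screen through the GMIP game instance.
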(event Custom|FocusOnWhiteBoardQuestion
  (bind _returnvalue (Sequencer|Player|CreateLevelSequencePlayer "/Game/Sequencer/FocusOnWhiteBoard.FocusOnWhiteBoard"))
  (Sequencer|Player|Play _returnvalue :!class /Script/MovieScene.MovieSceneSequencePlayer)
  (bind _outactors (Actor|GetAllActorsOfClass "/Game/Blueprints/Actors/BP_WhiteBoard.BP_WhiteBoard_C"))
  (Default|SetTextonWhiteBoard (Utilities|Array|Get(acopy) _outactors)))

(event Custom|CheckAnswerTrueORFalse
  (params (?True :type Boolean))
  (Default|StudentChooseAnswer (Variables|Default|GetcurrentStd) ?True))

(event Custom|FoucusOnTarget
  ;[0 0 0 0.5] FocusAndUnfocus On Target
  (Default|FocusonStudent (Variables|Default|GetBp%20Camera_ref) (Variables|Default|GetcurrentStd))
  ;[0 0 0 0.5] UpdateUI (Good/Bad Choice)
  ; UpdateSalary
  ; Update Progress bar
  ; Add BG Effect (True/False)
  (Utilities|FlowControl|Sequence
    (:then_0
      (EventDispatchers|BindEventtoOnChoice (Variables|Default|GetcurrentStd) (delegate Custom|CustomEvent)))
    (:then_1
      (EventDispatchers|BindEventtoOnBadChoice (Variables|Default|GetcurrentStd) (delegate Custom|CustomEvent_0)))))

(event Custom|BackToLocation
  ;[0 0 0 0.5] FocusAndUnfocus On Target
  (Default|UnFocusStudents (Variables|Default|GetBp%20Camera_ref))
  (if (not (Variables|Default|GetCanUnfocusOnStudent))
    (bind _returnvalue (Actor|GetActorOfClass "/Script/Engine.CameraActor"))
    (Utilities|FlowControl|Delay 2.2)
    (Game|Player|SetViewTargetwithBlend self _returnvalue 1.0 "VTBlend_Cubic" 0.0 false)
    (Widget|RemovefromParent (Variables|Default|GetGamePlayWBP_ref))
    (Utilities|FlowControl|Delay 0.8)
    (bind _asgmip (Utilities|Casting|CastToGMIP (Game|GetGameInstance)))
    (Default|CompleteDayDisplay _asgmip)
    (Default|CreateandViewLevelCompleateScreen _asgmip)))

(event Custom|FindStudentAnswer
  (params (true :type Boolean))
  ;[0 0 0 0.5] CheckStudentsAnswer
  (Default|CheckAnswer (Variables|Default|GetcurrentStd) true))

(event Custom|CustomEvent
  ;[0 0 0 0.5] UpdateUI (Good/Bad Choice)
  ; UpdateSalary
  ; Update Progress bar
  ; Add BG Effect (True/False)
  (Variables|Default|SetGood/BadChoice "/Game/Assets/UI/nt841.nt841")
  (Variables|Default|SetBG_True/FalseTexture "/Game/Assets/UI/R1.R1")
  (if (Variables|Default|GetCanUnfocusOnStudent)
    (Variables|Default|SetProgress (+ (Variables|Default|GetProgress) 0.25))
    (else
      (Variables|Default|SetProgress 1.0)))
  (Default|SetGood/BadChoiceImageandProgressBar (Variables|Default|GetGamePlayWBP_ref) (Variables|Default|GetProgress) (Variables|Default|GetGood/BadChoice) (Variables|Default|GetBG_True/FalseTexture)))

(event Custom|CustomEvent_0
  ;[0 0 0 0.5] UpdateUI (Good/Bad Choice)
  ; UpdateSalary
  ; Update Progress bar
  ; Add BG Effect (True/False)
  (Variables|Default|SetGood/BadChoice "/Game/Assets/UI/bad-logo-860-5068.bad-logo-860-5068")
  (Variables|Default|SetBG_True/FalseTexture "/Game/Assets/UI/R.R")
  (if (Variables|Default|GetCanUnfocusOnStudent)
    (Variables|Default|SetProgress (+ (Variables|Default|GetProgress) 0.25))
    (else
      (Variables|Default|SetProgress 1.0)))
  (Default|SetGood/BadChoiceImageandProgressBar (Variables|Default|GetGamePlayWBP_ref) (Variables|Default|GetProgress) (Variables|Default|GetGood/BadChoice) (Variables|Default|GetBG_True/FalseTexture)))

(event EventBeginPlay
  ;[0 0 0 0.5] enableInputs, user widget and get a refference of a teacher class
  (Variables|/Script/Engine.PlayerController|SetbShowMouseCursor self true)
  (bind _returnvalue (UserInterface|CreateWidget "/Game/UserWidget/gamePlayerWBPlevel01.gamePlayerWBPlevel01_C" 0 0))
  (bind _output_get (Variables|Default|SetGamePlayWBP_ref _returnvalue))
  (UserInterface|Viewport|AddtoViewport _output_get 0)
  (bind _asbp_camera (Utilities|Casting|CastToBP_Camera (Game|Player|GetPlayerPawn 0)))
  (Variables|Default|SetBp%20Camera_ref _asbp_camera)
  (bind _returnvalue_2 (Actor|GetActorOfClass "/Game/CoreComponents/StudentAndCameraInteraction.StudentAndCameraInteraction_C"))
  (Variables|Default|SetST_ActorRef _returnvalue_2))

(fn ConstructionScript)