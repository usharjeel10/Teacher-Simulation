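; BP_Lamp_01 is a placeable lamp prop from the JapaneseSchool assets, configured entirely in its construction script.
; Exposed-style variables set the intensity, attenuation radius and color temperature of its light component E.
; A dynamic instance of MI_Lamp_Emissive on the third material slot of SMLamp03 takes the same intensity as its Emissive parameter, tying glow to brightness.
; The event graph has no active logic.
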(event EventBeginPlay)

(event Collision|EventActorBeginOverlap
  (params (OtherActor :type Actor%20Object%20Reference)))

(event EventTick
  (params (DeltaSeconds :type Float%20%28single-precision%29)))

(fn ConstructionScript
  (bind _e (Variables|Default|Gete))
  (bind _intensity (Variables|Default|GetIntensity))
  (Rendering|Components|Light|SetIntensity _e _intensity)
  (Rendering|Lighting|SetAttenuationRadius _e (Variables|Default|GetNew%20Radius))
  (Class|LightComponent|SetTemperature _e (Variables|Default|GetNew%20Temperature))
  (bind _returnvalue (Rendering|Material|CreateDynamicMaterialInstance (Variables|Default|GetSM_Lamp_03) 2 "/Game/Assets/JapaneseSchool/Materials/Prop/MI_Lamp_Emissive.MI_Lamp_Emissive" "None" :!class /Script/Engine.PrimitiveComponent))
  (Rendering|Material|SetScalarParameterValue _returnvalue "Emissive" _intensity :!class /Script/Engine.MaterialInstanceDynamic))