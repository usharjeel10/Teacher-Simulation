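; PC_Level2 is the player controller for classroom teacher levels, supporting both the Level02 and Level03 teacher pawns.
; BeginPlay sets up input, cursor and the gameplay widget, caches the pawn, and hides interaction UI for Level03.
; testStart loops a timer that sets a shuffle-picked student's cheating state and informs the Level02 teacher.
; MoveToTheStds flip-flops the Level03 teacher between successive students and its return position, re-triggering after each return.
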(event Custom|cheatStudent
  ;[0 0 0 0.5] testStart
  (Utilities|Array|Shuffle (Variables|Default|Getshuffle))
  (bind _outactors (Actor|GetAllActorsOfClass "/Game/Blueprints/Student/StudentBP.StudentBP_C"))
  (Default|StudentStateinClassroom (Utilities|Array|Get(acopy) _outactors (Utilities|Array|Get(acopy) (Variables|Default|Getshuffle))) "NewEnumerator1")
  (Default|GetCheatingStd (Variables|Default|GetBp_Teache_%20Level02_ref) (Utilities|Array|Get(acopy) _outactors (Utilities|Array|Get(acopy) (Variables|Default|Getshuffle)))))

(event Custom|MoveToTheStds
  (Utilities|FlowControl|FlipFlop
    (:A
      (if (< (Variables|Default|GetGetStdToCheckActivity) 3)
        (Default|MovetotheStudent (Variables|Default|GetBp%20Teacher%20Level%2003_ref) (Variables|Default|GetGetStdToCheckActivity))
        (bind _result (Math|Integer|IncrementInt (Variables|Default|GetGetStdToCheckActivity))
          (:%20%20
            (Variables|Default|SetGetStdToCheckActivity _result)))))
    (:B
      (Default|TeacherBacktoCurrentPosition (Variables|Default|GetBp%20Teacher%20Level%2003_ref))
      (Utilities|FlowControl|Delay 2.0)
      (CallFunction|MovetotheStds))))

(event Custom|testStart
  ;[0 0 0 0.5] testStart
  (Utilities|Time|SetTimerbyEvent (delegate Custom|cheatStudent) 5.0 true))

(event EventBeginPlay
  ;[0 0 0 0.5] enableInputs, user widget and get a refference of a teacher class
  (Input|AddMappingContext (PlayerController|LocalPlayerSubsystems|GetEnhancedInputLocalPlayerSubsystem self) "/Game/inputs/IAM_Teacher.IAM_Teacher" 0 "(bIgnoreAllPressedKeysUntilRelease=True,bForceImmediately=False,bNotifyUserSettings=False)")
  (Variables|/Script/Engine.PlayerController|SetbShowMouseCursor self true)
  (bind _returnvalue (UserInterface|CreateWidget "/Game/UserWidget/GamePlayWBP_Level02.GamePlayWBP_Level02_C"))
  (bind _output_get (Variables|Default|SetGamePlayWBP_lvl02_ref _returnvalue))
  (UserInterface|Viewport|AddtoViewport _output_get 0)
  (bind _asbp_teacher_level_02 (Utilities|Casting|CastTobp_Teacher_Level02 (Game|Player|GetPlayerPawn 0))
    (:then
      (Variables|Default|SetBp_Teache_%20Level02_ref _asbp_teacher_level_02))
    (:CastFailed
      (bind _asbp_teacher_level_03 (Utilities|Casting|CastTobp_Teacher_Level03 (Game|Player|GetPlayerPawn 0)))
      (Variables|Default|SetBp%20Teacher%20Level%2003_ref _asbp_teacher_level_03)
      (Default|HideInteractionUI (Variables|Default|GetGamePlayWBP_lvl02_ref)))))

(fn ConstructionScript)