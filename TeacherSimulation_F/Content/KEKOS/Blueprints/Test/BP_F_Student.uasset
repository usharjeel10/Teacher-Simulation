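; Modular student character Blueprint that assembles its appearance in the construction script from mesh, material and color variables.
; Name prefixes switch between split torso/legs and a full-torso mesh, show torso props, and select cap-compatible hair.
; Dynamic materials tint hair, eyes, brows and glasses, and apply shared skin with detail textures.
; Skeletal parts follow HEAD via leader pose; BeginPlay is empty, leaving its animation call disconnected.
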(event EventBeginPlay)

(fn ConstructionScript
  (CallFunction|Construct)
  (Utilities|Array|Shuffle (Variables|Default|GetRandomStudentWuniform)))

(fn Construct
  (bind _torso (Variables|Default|GetTORSO))
  (bind _head (Variables|Default|GetHEAD))
  (bind _legs (Variables|Default|GetLEGS))
  (bind _hands (Variables|Default|GetHANDS))
  (bind _feets (Variables|Default|GetFEETS))
  (bind _eyebrows (Variables|Default|GetEYEBROWS))
  (bind _hair (Variables|Default|GetHAIR))
  (bind _cap2 (Variables|Default|GetCAP2))
  (bind _hands_2 (Variables|Default|GetHANDS))
  (bind _feets_2 (Variables|Default|GetFEETS))
  (bind _hair_2 (Variables|Default|GetHAIR))
  (bind _glasses (Variables|Default|GetGLASSES))
  (bind _full_torso (Variables|Default|GetFULL_TORSO))
  (bind _torsopropmesh (Variables|KEKOS|GetTorsoPropMesh))
  (bind _torso_prop (Variables|Default|GetTORSO_PROP))
  (bind _fulltorsomesh (Variables|KEKOS|GetFullTorsoMesh))
  (bind _skindetail (Variables|KEKOS|GetSkinDetail))
  (bind _cap2_2 (Variables|Default|GetCAP2))
  (bind _glasses_2 (Variables|Default|GetGLASSES))
  (Collision|SetCollisionEnabled (Variables|Default|GetCapsule) (Variables|KEKOSOthers|GetCollisionType))
  ;[0.5654 0.667 1] TORSO
  (Components|SkinnedMesh|SetSkinnedAssetandUpdate _torso (Variables|KEKOS|GetTorsoMesh) true)
  (Rendering|Material|SetMaterial _torso 1 (Variables|KEKOS|GetTorsoMaterial))
  (Rendering|SetVisibility (Variables|Default|GetTORSO) (not (Utilities|String|StartsWith (Utilities|GetDisplayName (Variables|KEKOS|GetFullTorsoMesh)) (LocalVariables|GetFullTorsoPrefix))) false)
  ;[0.5654 0.667 1] LEGS
  (Components|SkinnedMesh|SetSkinnedAssetandUpdate _legs (Variables|KEKOS|GetLegsMesh) true)
  (Rendering|Material|SetMaterial _legs 1 (Variables|KEKOS|GetLegsMaterial))
  (Rendering|SetVisibility (Variables|Default|GetLEGS) (not (Utilities|String|StartsWith (Utilities|GetDisplayName (Variables|KEKOS|GetFullTorsoMesh)) (LocalVariables|GetFullTorsoPrefix))) false)
  ;[0.5654 0.667 1] FULL TORSO
  (Components|SkinnedMesh|SetSkinnedAssetandUpdate _full_torso _fulltorsomesh true)
  (Rendering|Material|SetMaterial _full_torso 1 (Variables|KEKOS|GetFullTorsoMaterial))
  (Rendering|SetVisibility _full_torso (Utilities|String|StartsWith (Utilities|GetDisplayName _fulltorsomesh) (LocalVariables|GetFullTorsoPrefix)) false)
  ;[0.5654 0.667 1] HANDS
  (Components|SkinnedMesh|SetSkinnedAssetandUpdate _hands (Variables|KEKOS|GetHandsMesh) true)
  (Rendering|Material|SetMaterial _hands (Utilities|Array|LastIndex (Rendering|Material|GetMaterials _hands)) (Variables|KEKOS|GetHandsMaterial))
  ;[0.5654 0.667 1] FEET
  (Components|SkinnedMesh|SetSkinnedAssetandUpdate _feets (Variables|KEKOS|GetFeetsMesh) true)
  (Rendering|Material|SetMaterial _feets (Utilities|Array|LastIndex (Rendering|Material|GetMaterials _feets)) (Variables|KEKOS|GetFeetsMaterial))
  ;[0.5654 0.667 1] EYEBROWS
  (Components|SkinnedMesh|SetSkinnedAssetandUpdate _eyebrows (Variables|KEKOS|GetEyebrowsMesh) true)
  (bind _returnvalue (Rendering|Material|CreateDynamicMaterialInstance _eyebrows 0 0 "EyebrowsColor_Dynamic" :!class /Script/Engine.PrimitiveComponent))
  (Utilities|IsValid _returnvalue
    (:Is%20Valid
      (Rendering|Material|SetVectorParameterValue _returnvalue "D" (Math|Conversions|ToLinearColor(Color) (Variables|KEKOS|GetEyebrowsColor)) :!class /Script/Engine.MaterialInstanceDynamic))
    (:Is%20Not%20Valid
      _))
  ;[0.5654 0.667 1] EYES
  (Rendering|Material|SetMaterial _head 1 (Variables|KEKOS|GetEyesMaterial))
  (bind _returnvalue_2 (Rendering|Material|CreateDynamicMaterialInstance _head 1 0 "Eyes_Dynamic" :!class /Script/Engine.PrimitiveComponent))
  (Utilities|IsValid _returnvalue_2
    (:Is%20Valid
      (Rendering|Material|SetVectorParameterValue _returnvalue_2 "D_Color" (Math|Conversions|ToLinearColor(Color) (Variables|KEKOS|GetEyesColor)) :!class /Script/Engine.MaterialInstanceDynamic)
      (Rendering|Material|SetTextureParameterValue _returnvalue_2 "MASK" (.Value (Utilities|Map|Find (LocalVariables|GetEyesDetailToTexture) (Variables|KEKOS|GetEyesDetail)))))
    (:Is%20Not%20Valid
      _))
  ;[0.5654 0.667 1] GLASSES
  (Components|StaticMesh|SetStaticMesh _glasses (Variables|KEKOS|GetGlassesMesh))
  (Rendering|Material|SetMaterial _glasses 0 (Variables|KEKOS|GetGlassesMaterial))
  (bind _returnvalue_3 (Rendering|Material|CreateDynamicMaterialInstance _glasses 1 0 "Glass_Dynamic" :!class /Script/Engine.PrimitiveComponent))
  (Utilities|IsValid _returnvalue_3
    (:Is%20Valid
      (Rendering|Material|SetVectorParameterValue _returnvalue_3 "Color" (Math|Conversions|ToLinearColor(Color) (Variables|KEKOS|GetGlassesGlassColor)) :!class /Script/Engine.MaterialInstanceDynamic))
    (:Is%20Not%20Valid
      _))
  (Utilities|IsValid (Variables|/Script/Engine.StaticMeshComponent|GetStaticMesh _glasses_2)
    (:Is%20Valid
      (Rendering|SetVisibility _glasses_2 true false))
    (:Is%20Not%20Valid
      (Rendering|SetVisibility _glasses_2 false false)
      (Components|StaticMesh|SetStaticMesh _glasses_2 "/Engine/BasicShapes/Cube.Cube") ; Add some mesh to avoid null static mesh warning on build light
    ))
  ;[0.5654 0.667 1] CAP
  (Components|StaticMesh|SetStaticMesh _cap2_2 (Variables|KEKOS|GetCapMesh))
  (Rendering|Material|SetMaterial _cap2_2 0 (Variables|KEKOS|GetCapMaterial))
  (Utilities|IsValid (Variables|/Script/Engine.StaticMeshComponent|GetStaticMesh _cap2)
    (:Is%20Valid
      (Rendering|SetVisibility _cap2 true false))
    (:Is%20Not%20Valid
      (Rendering|SetVisibility _cap2 false false)
      (Components|StaticMesh|SetStaticMesh _cap2 "/Engine/BasicShapes/Cube.Cube") ; Add some mesh to avoid null static mesh warning on build light
    ))
  ;[0.5654 0.667 1] TORSO PROP
  (Components|SkinnedMesh|SetSkinnedAssetandUpdate _torso_prop _torsopropmesh true)
  (Rendering|Material|SetMaterial _torso_prop 0 (Variables|KEKOS|GetTorsoPropMaterial))
  (Rendering|SetVisibility _torso_prop (Utilities|String|StartsWith (Utilities|GetDisplayName _torsopropmesh) (LocalVariables|GetTorsoPropPrefix)) false)
  ;[0.5654 0.667 1] HAIR
  (Components|StaticMesh|SetStaticMesh _hair (.Value (Utilities|Map|Find (Variables|KEKOS|GetHairMesh) (Utilities|String|SelectString "WITHCAP" "FULL" (Utilities|String|StartsWith (Utilities|GetDisplayName (Variables|KEKOS|GetCapMesh)) (LocalVariables|GetCapPrefix))))))
  (bind _returnvalue_4 (Rendering|Material|CreateDynamicMaterialInstance _hair 0 0 "Hair_Dynamic" :!class /Script/Engine.PrimitiveComponent))
  (Utilities|IsValid _returnvalue_4
    (:Is%20Valid
      (Rendering|Material|SetVectorParameterValue _returnvalue_4 "D_Color" (Math|Conversions|ToLinearColor(Color) (Variables|KEKOS|GetHairColor)) :!class /Script/Engine.MaterialInstanceDynamic))
    (:Is%20Not%20Valid
      _))
  (Rendering|SetVisibility (Variables|Default|GetHAIR) (not (Utilities|String|StartsWith (Utilities|GetDisplayName (Variables|KEKOS|GetCapMesh)) (LocalVariables|GetFullCapPrefix))) false)
  (Utilities|IsValid (Variables|/Script/Engine.StaticMeshComponent|GetStaticMesh _hair_2)
    (:Is%20Valid
      (Rendering|SetVisibility _hair_2 true false))
    (:Is%20Not%20Valid
      (Rendering|SetVisibility _hair_2 false false)
      (Components|StaticMesh|SetStaticMesh _hair_2 "/Engine/BasicShapes/Cube.Cube") ; Add some mesh to avoid null static mesh warning on build light
    ))
  ;[0.5654 0.667 1] SKIN
  (bind _returnvalue_5 (Rendering|Material|CreateDynamicMaterialInstance (Variables|KEKOS|GetSkinMaterial) "Skin_Dynamic" "None" :!class /Script/Engine.KismetMaterialLibrary))
  (Rendering|Material|SetMaterial (Variables|Default|GetHEAD) 0 _returnvalue_5)
  (if (Class|MeshComponent|IsMaterialSlotNameValid _hands_2 (LocalVariables|GetSkinMaterialName))
    (Rendering|Material|SetMaterial _hands_2 0 _returnvalue_5))
  (if (Class|MeshComponent|IsMaterialSlotNameValid _feets_2 (LocalVariables|GetSkinMaterialName))
    (Rendering|Material|SetMaterial _feets_2 0 _returnvalue_5))
  (Utilities|IsValid _returnvalue_5
    (:Is%20Valid
      (Rendering|Material|SetTextureParameterValue _returnvalue_5 "Detail_Mask" (.Value (Utilities|Map|Find (LocalVariables|GetSkinDetailToMaskTexture) _skindetail)))
      (Rendering|Material|SetTextureParameterValue _returnvalue_5 "Detail_D" (.Value (Utilities|Map|Find (LocalVariables|GetSkinDetailToDiffuseTexture) _skindetail)))
      (Rendering|Material|SetTextureParameterValue _returnvalue_5 "Detail_EMI" (.Value (Utilities|Map|Find (LocalVariables|GetSkinDetailToEmissiveTexture) _skindetail)))
      (Rendering|Material|SetVectorParameterValue _returnvalue_5 "Detail_EMI_Color" (Math|Conversions|ToLinearColor(Color) (.Value (Utilities|Map|Find (LocalVariables|GetSkinDetailToEmissiveColor) _skindetail))) :!class /Script/Engine.MaterialInstanceDynamic))
    (:Is%20Not%20Valid
      _))
  ;[0.5654 0.667 1] ANIMATION
  (Components|SkinnedMesh|SetLeaderPoseComponent (Variables|Default|GetTorso_Prop) (Variables|Default|GetHead) true false))